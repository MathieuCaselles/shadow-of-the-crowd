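; King-of-the-hill capture point that the hero claims by staying inside its collision sphere.
; While occupied, pillar fires and lights turn on and a tick-delayed macro loop moves and spins the sphere mesh toward an offset.
; Leaving shuts off the effects and reverses progress until the sphere resets.
; Completion fires once, increments the GameInstance cleared count, plays shockwave and sound, recolors pillars and updates the hero's orb UI.
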(event `self.ReceiveBeginPlay`
  (bind _sm_sphere (`self.SM_Sphere`))
  (set `self.StartPosSphere` (`SceneComponent.K2_GetComponentLocation` _sm_sphere))
  (set `self.StartRotSphere` (`SceneComponent.K2_GetComponentRotation` _sm_sphere))
  (bind _assot_c_game_instance (cast `/Game/TMPS/TMPS_Art/BaDum/UI_UX/SotC_GameInstance` (`GameplayStatics.GetGameInstance`)))
  (set `self.RefGameInstance` _assot_c_game_instance))

(event `self.CollisionSphere.OnComponentBeginOverlap`
  (params (OverlappedComponent :type "PrimitiveComponent Object Reference") (OtherActor :type "Actor Object Reference") (OtherComp :type "PrimitiveComponent Object Reference") (OtherBodyIndex :type Integer) (bFromSweep :type Boolean) (SweepResult :type "HitResult Structure (by ref)"))
  (if (== OtherActor (`self.HeroCharacter`))
    (`|ExecutionSequence`
      (:`then_0`
        (`self.MoveAndRotateKOTH` (`self.SM_Sphere`) (`self.MovementVector`) (`self.MovementRotator`) (`self.TimeForCompletion`) :!label _label
          (:`Completed`
            (if (!= (`self.StartPosSphere`) (`SceneComponent.K2_GetComponentLocation` (`self.SM_Sphere`)) :`ErrorTolerance` 0.1)
              (`/Engine/EditorBlueprintResources/StandardMacros.DoOnce` false
                (:`Completed`
                  (set `self.Captured?` true)
                  (`/Engine/EditorBlueprintResources/StandardMacros.IncrementInt` (`/Game/TMPS/TMPS_Art/BaDum/UI_UX/SotC_GameInstance.NumberOfClearedKOTH` (`self.RefGameInstance`))
                    (:`  `
                      (`NiagaraFunctionLibrary.SpawnSystemAtLocation` "/Game/TMPS/TMPS_Art/BaDum/FX/SphereCapture/PS_ShockWaveKOTH.PS_ShockWaveKOTH" (`SceneComponent.K2_GetComponentLocation` (`self.DefaultSceneRoot`)))
                      (`GameplayStatics.PlaySoundAtLocation` "/Game/Magic___Spell_Sounds_PRO/downers-003.downers-003" (0.0 0.0 0.0) (struct) 1.0 1.0 0.0 null null null null)
                      (`FXSystemComponent.SetFloatParameter` (`self.PS_Tourbillon`) "Life" 0.0)
                      (for _array_element (`self.ListOfPillars`)
                        (`LightComponent.SetLightColor` (`/Game/BluePrints/BP_Pillar.Light` _array_element) (struct :`R` 1.0 :`G` 0.133929 :`A` 1.0) true)
                        (bind _ps_fire (`/Game/BluePrints/BP_Pillar.PS_Fire` _array_element))
                        (`FXSystemComponent.SetColorParameter` _ps_fire "Color" (struct :`R` 30.0 :`G` 6.349793 :`A` 1.0))
                        (`FXSystemComponent.SetColorParameter` _ps_fire "Color001" (struct :`R` 30.0 :`G` 6.239548 :`A` 1.0))
                        (`/Engine/EditorBlueprintResources/ActorMacros.Switch Has Authority`
                          (:`Authority`
                            (`/Game/TMPS/GAS/BP_HeroCharacter.UpdateOrbUI` (`self.HeroCharacter`)))))))))))))
      (:`then_1`
        (if (not (`self.Captured?`))
          (for _array_element_2 (`self.ListOfPillars`)
            (`LightComponent.SetIntensity` (`/Game/BluePrints/BP_Pillar.Light` _array_element_2) 7500.0)
            (bind _ps_fire_2 (`/Game/BluePrints/BP_Pillar.PS_Fire` _array_element_2))
            (`FXSystemComponent.SetFloatParameter` _ps_fire_2 "SpawnRateFire" 12.0)
            (`FXSystemComponent.SetFloatParameter` _ps_fire_2 "SpawnRateSparks" 20.0)
            (`FXSystemComponent.SetFloatParameter` (`self.PS_FireFlies`) "SpawnRate" 8.0)
            (`FXSystemComponent.SetFloatParameter` (`self.PS_Tourbillon`) "Life" 0.5)))))))

(event `self.CollisionSphere.OnComponentEndOverlap`
  (params (OverlappedComponent :type "PrimitiveComponent Object Reference") (OtherActor :type "Actor Object Reference") (OtherComp :type "PrimitiveComponent Object Reference") (OtherBodyIndex :type Integer))
  (if (== (`self.HeroCharacter`) OtherActor)
    (`|ExecutionSequence`
      (:`then_0`
        (goto _label :!via `Out`))
      (:`then_1`
        (if (not (`self.Captured?`))
          (for _array_element (`self.ListOfPillars`)
            (`LightComponent.SetIntensity` (`/Game/BluePrints/BP_Pillar.Light` _array_element) 0.0)
            (bind _ps_fire (`/Game/BluePrints/BP_Pillar.PS_Fire` _array_element))
            (`FXSystemComponent.SetFloatParameter` _ps_fire "SpawnRateFire" 0.0)
            (`FXSystemComponent.SetFloatParameter` _ps_fire "SpawnRateSparks" 0.0)
            (`FXSystemComponent.SetFloatParameter` (`self.PS_FireFlies`) "SpawnRate" 0.0)
            (`FXSystemComponent.SetFloatParameter` (`self.PS_Tourbillon`) "Life" 0.0)))))))

(fn `CalculationKOTH`
  (params (TargetLocation :type "Vector Structure") (NewParam :type "SceneComponent Object Reference"))
  (returns (NewLocation :type "Vector Structure") (NewRotation :type "Rotator Structure"))
  (return (`KismetMathLibrary.VLerp` (`self.StartPosSphere`) TargetLocation (`self.ProgressionTime`)) (`KismetMathLibrary.ComposeRotators` (`SceneComponent.K2_GetComponentRotation` NewParam) (* (`self.MovementRotator`) (/ (`GameplayStatics.GetWorldDeltaSeconds`) (`self.TimeForCompletion`))))))

(fn `FloatVectorToFloatRotator`
  (params (InputPin :type "Float (single-precision)"))
  (returns (ReturnValue :type "Float (double-precision)"))
  (return (select `bool` (>= (/ InputPin 90.0) 1.0) :`false` InputPin :`true` 90.0 :!type "Float (double-precision)")))

(fn `ResetPosAndRot`
  (params (Component :type "SceneComponent Object Reference"))
  (`SceneComponent.K2_SetWorldLocationAndRotation` Component (`self.StartPosSphere`) (`self.StartRotSphere`) false false))

(fn `UserConstructionScript`)