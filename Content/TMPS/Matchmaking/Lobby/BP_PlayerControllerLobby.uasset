(event `self.ReceiveBeginPlay`
  (set `self.bShowMouseCursor` true)
  (bind _returnvalue (`|CreateWidget` "/Game/TMPS/TMPS_Art/BaDum/UI_UX/W_Lobby_Menu.W_Lobby_Menu_C"))
  (bind _output_get (set `self.W_Lobby` _returnvalue))
  (`/Engine/EditorBlueprintResources/StandardMacros.IsValid` _output_get
    (:`Is Valid`
      (`UserWidget.AddToViewport` _output_get 0)
      (bind _returnvalue_2 (`GameplayStatics.GetActorOfClass` "/Game/TMPS/Matchmaking/Menu/BP_PawnMenu.BP_PawnMenu_C"))
      (`self.Possess` _returnvalue_2)
      (`/Engine/EditorBlueprintResources/ActorMacros.Switch Has Authority`
        (:`Remote`
          (bind _assot_c_game_instance (cast `/Game/TMPS/TMPS_Art/BaDum/UI_UX/SotC_GameInstance` (`GameplayStatics.GetGameInstance`)))
          (`/Game/TMPS/TMPS_Art/BaDum/UI_UX/W_Lobby_Menu.AddFriendToUI` (`self.W_Lobby`) "You" false (`KismetTextLibrary.Conv_StringToText` (`/Game/TMPS/TMPS_Art/BaDum/UI_UX/SotC_GameInstance.ServerJoinName` _assot_c_game_instance))))))))

(fn `AddFriendToUI`
  (params (FriendName :type Text) (HostName :type Text))
  (`/Game/TMPS/TMPS_Art/BaDum/UI_UX/W_Lobby_Menu.AddFriendToUI` (`self.W_Lobby`) FriendName (`self.HasAuthority`) HostName))

(fn `RemoveFriendToUi`
  (`/Game/TMPS/TMPS_Art/BaDum/UI_UX/W_Lobby_Menu.RemoveFriendToUI` (`self.W_Lobby`)))

(fn `UserConstructionScript`)