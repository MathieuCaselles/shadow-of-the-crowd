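; BP_GameModeLobby is the game mode for a two-player matchmaking lobby, handling players joining and leaving.
; On post-login it kicks anyone beyond two players with a "server full" message in French.
; When the second player joins, it re-applies the current session settings, then sends guest and host names to every lobby controller's UI.
; On logout every lobby controller removes the friend from its UI; hero spawning logic is left unconnected.
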(event `self.HandleStartingNewPlayer`
  (params (NewPlayer :type "PlayerController Object Reference")))

(event `self.K2_PostLogin`
  (params (NewPlayer :type "PlayerController Object Reference"))
  (bind _playerarray (`GameStateBase.PlayerArray` (`GameplayStatics.GetGameState`)))
  (bind _returnvalue (`KismetArrayLibrary.Array_Length` (`GameStateBase.PlayerArray` (`GameplayStatics.GetGameState`))))
  (if (> _returnvalue 2)
    (`AdvancedSessionsLibrary.KickPlayer` NewPlayer "Serveur complet")
    (elif (== _returnvalue 2)
      (bind (_numconnections _numprivateconnections _bislan _bisdedicated _ballowinvites _ballowjoininprogress _bisanticheatenabled _builduniqueid _extrasettings) (`AdvancedSessionsLibrary.GetSessionSettings`)
        (:`OnSuccess`
          (`UpdateSessionCallbackProxyAdvanced.UpdateSession` _extrasettings _numconnections
            (:`OnSuccess`
              (for _array_element _playerarray
                (bind _asbp_player_controller_lobby (cast `/Game/TMPS/Matchmaking/Lobby/BP_PlayerControllerLobby` (`PlayerState.GetPlayerController` _array_element)))
                (`/Game/TMPS/Matchmaking/Lobby/BP_PlayerControllerLobby.AddFriendToUI` _asbp_player_controller_lobby (`KismetTextLibrary.Conv_StringToText` (`AdvancedSessionsLibrary.GetPlayerName` NewPlayer)) (`KismetTextLibrary.Conv_StringToText` (`PlayerState.GetPlayerName` (`|GetArrayItem` _playerarray))))))))))))

(event `self.K2_OnLogout`
  (params (ExitingController :type "Controller Object Reference"))
  (bind _outactors (`GameplayStatics.GetAllActorsOfClass` "/Game/TMPS/Matchmaking/Lobby/BP_PlayerControllerLobby.BP_PlayerControllerLobby_C"))
  (for _array_element _outactors
    (`/Game/TMPS/Matchmaking/Lobby/BP_PlayerControllerLobby.RemoveFriendToUi` _array_element)))

(fn `UserConstructionScript`)