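; BP_EvilWall is a destructible wall that tracks the BP_EnemyCharacter until spawned, then rises from the ground with Niagara effects and sound.
; Tick drives the movement: it climbs to full height, waits, then sinks and destroys itself.
; Authority-side overlaps with fireballs and sword swipes reduce health, destroying the wall at zero.
; A floating health bar updates every tick and faces the player camera.
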(event `Spawn Wall`
  (bind (_returnvalue_x _returnvalue_y _returnvalue_z) (`KismetMathLibrary.BreakVector` (`self.K2_GetActorLocation`)))
  (bind _niagara2 (`self.Niagara2`))
  (bind _niagara3 (`self.Niagara3`))
  (bind _niagara (`self.Niagara`))
  (bind _niagara1 (`self.Niagara1`))
  (bind (_returnvalue_x_2 _returnvalue_y_2) (`KismetMathLibrary.BreakVector` (`SceneComponent.K2_GetComponentLocation` _niagara)))
  (bind (_returnvalue_x_3 _returnvalue_y_3) (`KismetMathLibrary.BreakVector` (`SceneComponent.K2_GetComponentLocation` _niagara3)))
  (bind (_returnvalue_x_4 _returnvalue_y_4) (`KismetMathLibrary.BreakVector` (`SceneComponent.K2_GetComponentLocation` _niagara1)))
  (bind (_returnvalue_x_5 _returnvalue_y_5) (`KismetMathLibrary.BreakVector` (`SceneComponent.K2_GetComponentLocation` _niagara2)))
  (set `self.bWaitingToSpawn` false)
  (set `self.heightMax` _returnvalue_z)
  (bind _output_get (set `self.heightMin` (- _returnvalue_z 290.0)))
  (`self.K2_SetActorLocation` (`KismetMathLibrary.MakeVector` _returnvalue_x _returnvalue_y _output_get) false true)
  (`PrimitiveComponent.SetCollisionEnabled` (`self.EvilWall`) "QueryAndPhysics")
  (`KismetSystemLibrary.Delay` 0.2)
  (`SceneComponent.K2_DetachFromComponent` (`self.Niagara1`) "KeepWorld" "KeepWorld" "KeepWorld" false)
  (`SceneComponent.K2_DetachFromComponent` (`self.Niagara2`) "KeepWorld" "KeepWorld" "KeepWorld" false)
  (`SceneComponent.K2_DetachFromComponent` (`self.Niagara3`) "KeepWorld" "KeepWorld" "KeepWorld" false)
  (`SceneComponent.K2_DetachFromComponent` (`self.Niagara`) "KeepWorld" "KeepWorld" "KeepWorld" false)
  (`SceneComponent.K2_SetWorldLocation` _niagara1 (`KismetMathLibrary.MakeVector` _returnvalue_x_4 _returnvalue_y_4 (`self.heightMax`)) false true)
  (`SceneComponent.K2_SetWorldLocation` _niagara2 (`KismetMathLibrary.MakeVector` _returnvalue_x_5 _returnvalue_y_5 (`self.heightMax`)) false true)
  (`SceneComponent.K2_SetWorldLocation` _niagara3 (`KismetMathLibrary.MakeVector` _returnvalue_x_3 _returnvalue_y_3 (`self.heightMax`)) false true)
  (`SceneComponent.K2_SetWorldLocation` _niagara (`KismetMathLibrary.MakeVector` _returnvalue_x_2 _returnvalue_y_2 (`self.heightMax`)) false true)
  (`ActorComponent.Activate` (`self.Niagara2`) false)
  (`ActorComponent.Activate` (`self.Niagara3`) false)
  (`ActorComponent.Activate` (`self.Niagara`) false)
  (`ActorComponent.Activate` (`self.Niagara1`) false)
  (`GameplayStatics.PlaySoundAtLocation` "/Game/Magic___Spell_Sounds_PRO/Elements___School/Nature/wav/Nature_Spell_5.Nature_Spell_5" (`self.K2_GetActorLocation`) (struct) 1.0 1.0 0.0 null null null null)
  (`SceneComponent.SetHiddenInGame` (`self.EvilWall`) false true))

(event `self.ReceiveBeginPlay`
  (bind _asfloating_health_bar (cast `/Game/TMPS/TMPS_Art/BaDum/UI_UX/FloatingHealthBar` (`WidgetComponent.GetWidget` (`self.HealthBarWidget`))))
  (set `self.FloatingHealthBar` _asfloating_health_bar)
  (`PrimitiveComponent.SetCollisionEnabled` (`self.EvilWall`) "NoCollision")
  (bind _returnvalue (`GameplayStatics.GetActorOfClass` "/Game/TMPS/GAS/BP_EnemyCharacter.BP_EnemyCharacter_C"))
  (set `self.Enemy` _returnvalue)
  (`/Engine/EditorBlueprintResources/ActorMacros.Switch Has Authority`
    (:`Remote`
      (`SceneComponent.SetHiddenInGame` (`self.EvilWall`) false false))))

(event `self.ReceiveTick`
  (params (DeltaSeconds :type "Float (single-precision)"))
  (bind (_returnvalue_x _returnvalue_y _returnvalue_z) (`KismetMathLibrary.BreakVector` (`self.K2_GetActorLocation`)))
  (bind (_returnvalue_x_2 _returnvalue_y_2 _returnvalue_z_2) (`KismetMathLibrary.BreakVector` (`self.K2_GetActorLocation`)))
  (bind (_returnvalue_x_3 _returnvalue_y_3 _returnvalue_z_3) (`KismetMathLibrary.BreakVector` (`self.K2_GetActorLocation`)))
  (bind (_returnvalue_x_4 _returnvalue_y_4 _returnvalue_z_4) (`KismetMathLibrary.BreakVector` (`self.K2_GetActorLocation`)))
  (bind _returnvalue (`self.GetTransform` (`self.Enemy`)))
  (`self.UpdateFLoatingBar` (/ (`self.CurrentHealth`) (`self.MaxHealth`)))
  (set `self.DeltaSeconds` DeltaSeconds)
  (if (`self.bWaitingToSpawn`)
    (`self.K2_SetActorLocationAndRotation` (`KismetMathLibrary.MakeVector` (.x (.location _returnvalue)) (.y (.location _returnvalue)) (- (.z (.location _returnvalue)) 90.0)) (.rotation _returnvalue) false true)
    (elif (`self.bCanDespawn`)
      (`self.K2_SetActorLocation` (`KismetMathLibrary.MakeVector` _returnvalue_x_3 _returnvalue_y_3 (- _returnvalue_z_3 (* (`self.SpeedWall`) (`self.DeltaSeconds`)))) false true)
      (if (<= _returnvalue_z (`self.heightMin`))
        (`self.K2_DestroyActor`))
      (elif (< _returnvalue_z_4 (`self.heightMax`))
        (`self.K2_SetActorLocation` (`KismetMathLibrary.MakeVector` _returnvalue_x_2 _returnvalue_y_2 (+ _returnvalue_z_2 (* (`self.SpeedWall`) (`self.DeltaSeconds`)))) false true)
        (elif (not (`self.bStartDelayDespawn`))
          (set `self.bStartDelayDespawn` true)
          (`ActorComponent.SetActive` (`self.Niagara1`) false true)
          (`ActorComponent.SetActive` (`self.Niagara2`) false true)
          (`ActorComponent.SetActive` (`self.Niagara3`) false true)
          (`ActorComponent.SetActive` (`self.Niagara`) false true)
          (`KismetSystemLibrary.Delay` (`self.DelayWall`))
          (set `self.bCanDespawn` true)
          (`ActorComponent.Activate` (`self.Niagara2`) false)
          (`ActorComponent.Activate` (`self.Niagara3`) false)
          (`ActorComponent.Activate` (`self.Niagara`) false)
          (`ActorComponent.Activate` (`self.Niagara1`) false)
          (`GameplayStatics.PlaySoundAtLocation` "/Game/Magic___Spell_Sounds_PRO/Elements___School/Nature/wav/Nature_Spell_5.Nature_Spell_5" (`self.K2_GetActorLocation`) (struct) 1.0 1.0 0.0 null null null null))))))

(event `self.ReceiveActorBeginOverlap`
  (params (OtherActor :type "Actor Object Reference"))
  (`/Engine/EditorBlueprintResources/ActorMacros.Switch Has Authority`
    (:`Authority`
      ;[1 1 1] ON OVERLP
      (`|ExecutionSequence`
        (:`then_0`
          (cast `/Game/TMPS/GAS/Abilities/Characters/Hero/SummonFireBall/BP_FireBall` OtherActor)
          (`self.UpdateHealth` (- (`self.CurrentHealth`) 1.0)))
        (:`then_1`
          (cast `/Game/TMPS/GAS/Abilities/Characters/Hero/AttackWithSword/BP_SwordSwipe` OtherActor)
          (`self.UpdateHealth` (- (`self.CurrentHealth`) 7.0)))))))

(event `UpdateHealth`
  (params (newhealth :type "Float (double-precision)"))
  ;[1 1 1] ON OVERLP
  (set `self.CurrentHealth` newhealth)
  (if (<= (`self.CurrentHealth`) 0.0)
    (`GameplayStatics.PlaySoundAtLocation` "/Game/Magic___Spell_Sounds_PRO/Elements___School/Nature/wav/Nature_Spell_1.Nature_Spell_1" (`self.K2_GetActorLocation`) (struct) 1.2 1.0 0.0 null null null null)
    (`self.K2_DestroyActor`)
    (else
      (`GameplayStatics.PlaySoundAtLocation` "/Game/Magic___Spell_Sounds_PRO/Elements___School/Nature/wav/Nature_Spell_10_1.Nature_Spell_10_1" (`self.K2_GetActorLocation`) (struct) 0.4 1.0 0.0 null null null null))))

(event `UpdateFLoatingBar`
  (params (percent :type "Float (double-precision)"))
  (bind _healthbarwidget (`self.HealthBarWidget`))
  ;[1 1 1] ui
  (`ProgressBar.SetPercent` (`/Game/TMPS/TMPS_Art/BaDum/UI_UX/FloatingHealthBar.ProgressBarHealth` (`self.FloatingHealthBar`)) percent)
  (`SceneComponent.K2_SetWorldRotation` _healthbarwidget (`KismetMathLibrary.FindLookAtRotation` (`SceneComponent.K2_GetComponentLocation` _healthbarwidget) (`SceneComponent.K2_GetComponentLocation` (`PlayerCameraManager.TransformComponent` (`GameplayStatics.GetPlayerCameraManager` 0)))) false false))

(fn `UserConstructionScript`)