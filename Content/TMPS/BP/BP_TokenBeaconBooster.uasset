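; BP_TokenBeaconBooster is a token actor that mirrors a BeaconBomb's position at an offset, apparently for the BBEG's map.
; On BeginPlay it caches BP_BDTGameState, then each Tick teleports to the bomb's capsule location, shifted along Y by the game state's BBEGMapOffset.
; Once the BeaconBomb reference is invalid, EndGame disables ticking and destroys the token.
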(event `self.ReceiveBeginPlay`
  ;[1 1 1] Get Game State
  (bind _asbp_bdtgame_state (cast `/Game/TMPS/GAS/BP_BDTGameState` (`GameplayStatics.GetGameState`)))
  (set `self.BDTGameState` _asbp_bdtgame_state))

(event `self.ReceiveTick`
  (params (DeltaSeconds :type "Float (single-precision)"))
  (bind _beaconbomb (`self.BeaconBomb`))
  (bind (_returnvalue_x _returnvalue_y _returnvalue_z) (`KismetMathLibrary.BreakVector` (`SceneComponent.K2_GetComponentLocation` (`Character.CapsuleComponent` _beaconbomb))))
  ;[1 1 1] Set hero token position
  (`/Engine/EditorBlueprintResources/StandardMacros.IsValid` _beaconbomb
    (:`Is Valid`
      (`self.K2_SetActorLocation` (`KismetMathLibrary.MakeVector` _returnvalue_x (+ _returnvalue_y (`BDTGameState.BBEGMapOffset` (`self.BDTGameState`))) _returnvalue_z) false true))
    (:`Is Not Valid`
      (`self.EndGame`))))

(fn `EndGame`
  (`self.SetActorTickEnabled` false)
  (`self.K2_DestroyActor`))

(fn `UserConstructionScript`)