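; BP_HeroToken is an actor that mirrors the hero character's position at a Y offset, apparently onto a separate BBEG map.
; On BeginPlay it caches the BDT game state and finds the BP_HeroCharacter in the level.
; Each tick it teleports to the hero capsule's location, shifted by the game state's BBEGMapOffset.
; When the hero is no longer valid, EndGame turns off its tick.
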(event `self.ReceiveBeginPlay`
  ;[1 1 1] Get Game State
  (bind _asbp_bdtgame_state (cast `/Game/TMPS/GAS/BP_BDTGameState` (`GameplayStatics.GetGameState`)))
  (set `self.BDTGameState` _asbp_bdtgame_state)
  ;[1 1 1] Get HeroToken
  (bind _returnvalue (`GameplayStatics.GetActorOfClass` "/Game/TMPS/GAS/BP_HeroCharacter.BP_HeroCharacter_C"))
  (set `self.HeroCharacter` _returnvalue))

(event `self.ReceiveTick`
  (params (DeltaSeconds :type "Float (single-precision)"))
  (bind _herocharacter (`self.HeroCharacter`))
  (bind (_returnvalue_x _returnvalue_y _returnvalue_z) (`KismetMathLibrary.BreakVector` (`SceneComponent.K2_GetComponentLocation` (`Character.CapsuleComponent` _herocharacter))))
  ;[1 1 1] Set hero token position
  (`/Engine/EditorBlueprintResources/StandardMacros.IsValid` _herocharacter
    (:`Is Valid`
      (`self.K2_SetActorLocation` (`KismetMathLibrary.MakeVector` _returnvalue_x (+ _returnvalue_y (`BDTGameState.BBEGMapOffset` (`self.BDTGameState`))) _returnvalue_z) false true))
    (:`Is Not Valid`
      (`self.EndGame`))))

(fn `EndGame`
  (`self.SetActorTickEnabled` false))

(fn `UserConstructionScript`)