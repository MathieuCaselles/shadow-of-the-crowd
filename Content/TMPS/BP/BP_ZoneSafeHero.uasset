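; BP_ZoneSafeHero is an actor that forms a safe zone following the hero, suppressing the enemy's abilities inside it.
; On BeginPlay it caches the first hero and enemy characters found, then teleports itself to the hero's location every Tick.
; When that enemy begins overlapping the zone its abilities are blocked, and they are re-enabled when the overlap ends.
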(event `self.ReceiveBeginPlay`
  (bind _returnvalue (`GameplayStatics.GetActorOfClass` "/Game/TMPS/GAS/BP_HeroCharacter.BP_HeroCharacter_C"))
  (set `self.Hero` _returnvalue)
  (bind _returnvalue_2 (`GameplayStatics.GetActorOfClass` "/Game/TMPS/GAS/BP_EnemyCharacter.BP_EnemyCharacter_C"))
  (set `self.Enemy` _returnvalue_2))

(event `self.ReceiveTick`
  (params (DeltaSeconds :type "Float (single-precision)"))
  (bind _hero (`self.Hero`))
  (`/Engine/EditorBlueprintResources/StandardMacros.IsValid` _hero
    (:`Is Valid`
      (`self.K2_SetActorLocation` (`self.K2_GetActorLocation` _hero) false true))))

(event `self.ReceiveActorBeginOverlap`
  (params (OtherActor :type "Actor Object Reference"))
  (if (== OtherActor (`self.Enemy`))
    (`/Game/TMPS/GAS/BP_EnemyCharacter.BlockAbilities` (`self.Enemy`))))

(event `self.ReceiveActorEndOverlap`
  (params (OtherActor :type "Actor Object Reference"))
  (if (== OtherActor (`self.Enemy`))
    (`/Game/TMPS/GAS/BP_EnemyCharacter.EnableAbilities` (`self.Enemy`))))

(fn `UserConstructionScript`)