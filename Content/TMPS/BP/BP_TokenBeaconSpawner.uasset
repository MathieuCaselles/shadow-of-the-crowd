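; BP_TokenBeaconSpawner is a token actor meant to mirror a BeaconBomb's position, offset along Y by the game state's BBEG map offset.
; BeginPlay, Tick and EndGame are all empty, so none of its logic runs.
; Disconnected nodes hold the game state caching, the teleport to the bomb's capsule location, and the tick shutdown and destroy intended for when the bomb becomes invalid.
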(event `self.ReceiveBeginPlay`)

(event `self.ReceiveTick`
  (params (DeltaSeconds :type "Float (single-precision)"))
  ;[1 1 1] Set hero token position
)

(fn `EndGame`)

(fn `UserConstructionScript`)