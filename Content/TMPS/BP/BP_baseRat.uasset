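; Base rat enemy Blueprint that tracks health and dies when it runs out.
; The Damage event subtracts the incoming value from HP, then runs an alive check that spawns a death effect at the rat's location and destroys it at zero or below.
; A call notifying the enemy AI controller of spawning is left unconnected, and BeginPlay and Tick are empty.
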(event `self.ReceiveBeginPlay`)

(event `self.ReceiveTick`
  (params (DeltaSeconds :type "Float (single-precision)")))

(event `Damage`
  (params (`Damage Value` :type "Float (double-precision)"))
  (set `self.HP` (- (`self.HP`) `Damage Value`))
  (`self.isAlive`))

(event `isAlive`
  (if (not (> (`self.HP`) 0.0))
    (`NiagaraFunctionLibrary.SpawnSystemAtLocation` "/Game/TMPS/TMPS_Art/BaDum/FX/Death/PS_Death.PS_Death" (`self.K2_GetActorLocation`))
    (`self.K2_DestroyActor`)))

(fn `UserConstructionScript`)