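; BP_HeroCharacter is the playable hero, using GAS abilities for fireball summon, sword attack and lightning dash.
; BeginPlay disables input, resets game-instance data, grants abilities by array index, links KOTH and door actors, adds depth of field and triggers delayed mass spawning.
; Possession builds the HUD, while health changes notify UI and play haptic and blood-hit feedback.
; Destruction without a win notifies the door of the loss.
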(event `EnhancedInput|/Game/Inputs/HeroCharacter/Actions/IA_Look`
  (params (ActionValue :type "Vector2D Structure") (ElapsedSeconds :type "Float (double-precision)") (TriggeredSeconds :type "Float (double-precision)") (InputAction :type "InputAction Object Reference" :default "/Game/Inputs/HeroCharacter/Actions/IA_Look.IA_Look"))
  (bind _charactermovement (`self.CharacterMovement`))
  ;[1 1 1] Orient hero to direction if not use IA_Look
  (:`Started`
    (set `CharacterMovementComponent.bOrientRotationToMovement` false _charactermovement))
  (:`Completed`
    (set `CharacterMovementComponent.bOrientRotationToMovement` true _charactermovement)))

(event `self.ReceiveBeginPlay`
  (`self.DisableInput` (`GameplayStatics.GetPlayerController` 0))
  (bind _assot_c_game_instance (cast `/Game/TMPS/TMPS_Art/BaDum/UI_UX/SotC_GameInstance` (`GameplayStatics.GetGameInstance`)))
  (bind _output_get (set `self.GameInstance` _assot_c_game_instance))
  (`/Game/TMPS/TMPS_Art/BaDum/UI_UX/SotC_GameInstance.ResetData` _output_get)
  ;[1 1 1] Ne bouge plus
  ;;[0.2578 0 1] Add abilities in hero
  (`self.initializeAbilities`)
  (bind _outactors (`GameplayStatics.GetAllActorsOfClass` "/Game/BluePrints/BP_KOTH.BP_KOTH_C"))
  (for _array_element _outactors
    (set `/Game/BluePrints/BP_KOTH.HeroCharacter` self _array_element)
    (bind _returnvalue (`GameplayStatics.GetActorOfClass` "/Game/TMPS/TMPS_Art/BaDum/Mesh/Props/BP_Door.BP_Door_C"))
    (set `/Game/TMPS/TMPS_Art/BaDum/Mesh/Props/BP_Door.HeroCharacter` self _returnvalue))
  ;;[0.1145 1 0] Camera Tilt shift DOF
  (bind _returnvalue_2 (`AddComponent|NODE_AddPostProcessComponent-2`))
  (setmembers `PostProcessSettings` :`StructRef` (`PostProcessComponent.Settings` _returnvalue_2) :`DepthOfFieldFstop` 0.2 :`DepthOfFieldSensorWidth` 100.0 :`DepthOfFieldFocalDistance` (`SpringArmComponent.TargetArmLength` (`self.SpringArm`)))
  (`KismetSystemLibrary.Delay` 3.0)
  (`self.DoSpawnWithMassSwpawneur`))

(event `Key|SpaceBar`
  (params (Key :type "Key Structure"))
  ;[1 0.004673 0] TMPS DEBUG SWITCH TO BADUM
)

(event `Key|Gamepad_Special_Left`
  (params (Key :type "Key Structure"))
  ;[1 0.004673 0] TMPS DEBUG SWITCH TO BADUM
)

(event `InitHudHero`
  ;[1 1 1] Ne bouge plus
  (`KismetSystemLibrary.PrintString` "ALED")
  (`/Engine/EditorBlueprintResources/ActorMacros.Switch Has Authority`
    (:`Authority`
      (`KismetSystemLibrary.PrintString` "BAH ALORS")
      ;;[1 0.4462 0] ADD UI TO VIEWPORET
      (`WidgetLayoutLibrary.RemoveAllWidgets` :!label _label)
      (bind _asplayer_controller (cast `PlayerController` (stale `self.ReceivePossessed` NewController)))
      (set `PlayerController.bShowMouseCursor` false _asplayer_controller)
      (bind _returnvalue (`|CreateWidget` "/Game/TMPS/TMPS_Art/BaDum/UI_UX/Hero_UI_controller.Hero_UI_controller_C"))
      (`UserWidget.AddToViewport` _returnvalue 0)
      (bind _assot_c_game_instance (cast `/Game/TMPS/TMPS_Art/BaDum/UI_UX/SotC_GameInstance` (`self.GameInstance`)))
      (`/Game/TMPS/TMPS_Art/BaDum/UI_UX/SotC_GameInstance.SetWidget` _assot_c_game_instance _returnvalue))))

(event `self.ReceivePossessed`
  (params (NewController :type "Controller Object Reference"))
  ;[1 1 1] Ne bouge plus
  ;;[1 0.4462 0] ADD UI TO VIEWPORET
  (goto _label))

(event `EnhancedInput|/Game/Inputs/HeroCharacter/Actions/IA_SummonFireBall`
  (params (ActionValue :type Boolean) (ElapsedSeconds :type "Float (double-precision)") (TriggeredSeconds :type "Float (double-precision)") (InputAction :type "InputAction Object Reference" :default "/Game/Inputs/HeroCharacter/Actions/IA_SummonFireBall.IA_SummonFireBall"))
  ;[1 1 1] Ne bouge plus
  ;;[0.2578 0 1] Summon Fireball
  (:`Triggered`
    (`self.ActivateAbility` 0)))

(event `self.ReceiveUnpossessed`
  (params (OldController :type "Controller Object Reference"))
  ;[1 1 1] Ne bouge plus
  ;;[1 0.4462 0] REMOVE UI FROM VIEWPORT
  (`WidgetLayoutLibrary.RemoveAllWidgets`))

(event `self.OnHealthChanged`
  (params (oldValue :type "Float (single-precision)") (newValue :type "Float (single-precision)"))
  ;[1 1 1] Ne bouge plus
  ;;[1 0.4462 0] UPDATE UI HEALTH
  (`self.HeroCharacterHealthChangedDispatcher` (`KismetMathLibrary.FClamp` (/ newValue (`self.GetMaxHealth`))))
  (`/Engine/EditorBlueprintResources/ActorMacros.Switch Has Authority`
    (:`Authority`
      ;[0.4792 1 1] Retour Haptic + screen damage blood
      ;;[1 1 1] ok fonctionne
      (`ForceFeedbackComponent.Play` (`self.ForceFeedback`) 0.0)
      (`self.BloodHitWidget`
        (:`then`
          (if (not (`UserWidget.IsAnyAnimationPlaying` (`self.BloodHitWidget`)))
            (`/Game/TMPS/TMPS_Art/BaDum/UI_UX/w_blood.Play hit animation` (`self.BloodHitWidget`))))
        (:`else`
          (bind _returnvalue (`|CreateWidget` "/Game/TMPS/TMPS_Art/BaDum/UI_UX/w_blood.w_blood_C" (`GameplayStatics.GetPlayerController` 0)))
          (bind _output_get (set `self.BloodHitWidget` _returnvalue))
          (`UserWidget.AddToViewport` _output_get 0)
          (`/Game/TMPS/TMPS_Art/BaDum/UI_UX/w_blood.Play hit animation` (`self.BloodHitWidget`)))))))

(event `EnhancedInput|/Game/Inputs/HeroCharacter/Actions/IA_AttackWithSword`
  (params (ActionValue :type Boolean) (ElapsedSeconds :type "Float (double-precision)") (TriggeredSeconds :type "Float (double-precision)") (InputAction :type "InputAction Object Reference" :default "/Game/Inputs/HeroCharacter/Actions/IA_AttackWithSword.IA_AttackWithSword"))
  ;[1 1 1] Ne bouge plus
  ;;[0.2578 0 1] Attack With Sword
  (:`Started`
    (`self.ActivateAbility` 1)))

(event `UpdateOrbUI`
  ;[1 1 1] Ne bouge plus
  ;;[1 0.4462 0] UPDATE UI orb
  (`self.HeroCharacterUpdateOrb`))

(event `EnhancedInput|/Game/Inputs/HeroCharacter/Actions/IA_LightningDash`
  (params (ActionValue :type Boolean) (ElapsedSeconds :type "Float (double-precision)") (TriggeredSeconds :type "Float (double-precision)") (InputAction :type "InputAction Object Reference" :default "/Game/Inputs/HeroCharacter/Actions/IA_LightningDash.IA_LightningDash"))
  ;[1 1 1] Ne bouge plus
  ;;[0.2578 0 1] Lightning Dash
  (:`Started`
    (`self.ActivateAbility` 2)))

(event `self.ReceiveDestroyed`
  (if (not (`self.bHasWon`))
    (bind _returnvalue (`GameplayStatics.GetActorOfClass` "/Game/TMPS/TMPS_Art/BaDum/Mesh/Props/BP_Door.BP_Door_C"))
    (`/Engine/EditorBlueprintResources/StandardMacros.IsValid` _returnvalue
      (:`Is Valid`
        (`/Game/TMPS/TMPS_Art/BaDum/Mesh/Props/BP_Door.HeroLoose` _returnvalue)))))

(event `DoSpawnWithMassSwpawneur`
  (bind _returnvalue (`GameplayStatics.GetActorOfClass` "/Script/MassSpawner.MassSpawner"))
  (`/Engine/EditorBlueprintResources/StandardMacros.IsValid` _returnvalue
    (:`Is Valid`
      (`MassSpawner.DoSpawning` _returnvalue))))

(fn `initializeAbilities`
  (for (_array_element _array_index) (`self.Abilities`)
    (`self.GrantAbility` _array_element 1 _array_index)))

(fn `UserConstructionScript`)