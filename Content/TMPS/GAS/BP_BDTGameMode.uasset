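; BP_BDTGameMode is a game mode for a two-player session that pairs a hero against an enemy character, Badum.
; New players spawn and possess BP_HeroCharacter at start "0" while no hero exists, otherwise BP_EnemyCharacter at start "1".
; PostLogin kicks anyone beyond two players as server full.
; When the second joins, it updates the session using its current extra settings and connection count.
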(event `self.HandleStartingNewPlayer`
  (params (NewPlayer :type "PlayerController Object Reference"))
  ;[1 1 1] SetupPlayer Controller
  (if (not (`KismetSystemLibrary.IsValid` (`self.HeroLobbyP1`)))
    (bind _output_get (set `self.HeroController` NewPlayer))
    (bind _returnvalue (`|SpawnActorFromClass` "/Game/TMPS/GAS/BP_HeroCharacter.BP_HeroCharacter_C" (`self.GetTransform` (`self.K2_FindPlayerStart` _output_get "0")) "Undefined" "OverrideRootScale" null null))
    (bind _output_get_2 (set `self.HeroLobbyP1` _returnvalue))
    (`Controller.Possess` (`self.HeroController`) _output_get_2)
    (else
      (bind _output_get_3 (set `self.BadumController` NewPlayer))
      (bind _returnvalue_2 (`|SpawnActorFromClass` "/Game/TMPS/GAS/BP_EnemyCharacter.BP_EnemyCharacter_C" (`self.GetTransform` (`self.K2_FindPlayerStart` _output_get_3 "1")) "Undefined" "OverrideRootScale" null null))
      (bind _output_get_4 (set `self.Badum` _returnvalue_2))
      (`Controller.Possess` (`self.BadumController`) _output_get_4))))

(event `self.K2_PostLogin`
  (params (NewPlayer :type "PlayerController Object Reference"))
  (bind _returnvalue (`KismetArrayLibrary.Array_Length` (`GameStateBase.PlayerArray` (`GameplayStatics.GetGameState`))))
  ;[1 1 1] Manage max player
  (if (> _returnvalue 2)
    (`AdvancedSessionsLibrary.KickPlayer` NewPlayer "Serveur complet")
    (elif (== _returnvalue 2)
      (bind (_numconnections _numprivateconnections _bislan _bisdedicated _ballowinvites _ballowjoininprogress _bisanticheatenabled _builduniqueid _extrasettings) (`AdvancedSessionsLibrary.GetSessionSettings`)
        (:`OnSuccess`
          (`UpdateSessionCallbackProxyAdvanced.UpdateSession` _extrasettings _numconnections))))))

(fn `UserConstructionScript`)