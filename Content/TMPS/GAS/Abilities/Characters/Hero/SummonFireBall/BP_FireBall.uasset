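; Fireball projectile actor for the Hero's GAS abilities, with Niagara effects for cast, wall impact and rat hit.
; Overlaps ignore the instigator, KOTH and the first enemy character found at spawn; authority applies the damage effect spec to beacons with an ability system.
; Hits spawn a wall impact and destroy it.
; Destruction plays rat impact and death effects unless HasHitARat was cleared, which remote overlaps never do.
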(event `self.ReceiveBeginPlay`
  (`NiagaraFunctionLibrary.SpawnSystemAtLocation` "/Game/TMPS/TMPS_Art/BaDum/FX/FireBall/FireBall/PS_FireCast.PS_FireCast" (`self.K2_GetActorLocation`))
  (bind _returnvalue (`GameplayStatics.GetActorOfClass` "/Game/TMPS/GAS/BP_EnemyCharacter.BP_EnemyCharacter_C"))
  (set `self.BP_EnemyChar` _returnvalue))

(event `self.Collision.OnComponentBeginOverlap`
  (params (OverlappedComponent :type "PrimitiveComponent Object Reference") (OtherActor :type "Actor Object Reference") (OtherComp :type "PrimitiveComponent Object Reference") (OtherBodyIndex :type Integer) (bFromSweep :type Boolean) (SweepResult :type "HitResult Structure (by ref)"))
  (if (and (!= OtherActor (`self.GetInstigator`)) (!= (`GameplayStatics.GetObjectClass` OtherActor) "/Game/BluePrints/BP_KOTH.BP_KOTH_C") (!= OtherActor (`self.BP_EnemyChar`)))
    (`/Engine/EditorBlueprintResources/ActorMacros.Switch Has Authority`
      (:`Authority`
        (bind _asbdtbeacon_base (cast `BDTBeaconBase` OtherActor)
          (:`then`
            (bind _returnvalue (`AbilitySystemBlueprintLibrary.GetAbilitySystemComponent` _asbdtbeacon_base))
            (if (`KismetSystemLibrary.IsValid` _returnvalue)
              (`AbilitySystemComponent.BP_ApplyGameplayEffectSpecToSelf` _returnvalue (`self.DamageEffectSpecHandle`))
              (set `self.hasHitARat` false)
              (`self.K2_DestroyActor`)))
          (:`CastFailed`
            (set `self.hasHitARat` false)
            (`self.K2_DestroyActor`))))
      (:`Remote`
        (`self.K2_DestroyActor`)))))

(event `self.Collision.OnComponentHit`
  (params (HitComponent :type "PrimitiveComponent Object Reference") (OtherActor :type "Actor Object Reference") (OtherComp :type "PrimitiveComponent Object Reference") (NormalImpulse :type "Vector Structure") (Hit :type "HitResult Structure (by ref)"))
  (if (!= OtherActor (`self.BP_EnemyChar`))
    (`NiagaraFunctionLibrary.SpawnSystemAtLocation` "/Game/TMPS/TMPS_Art/BaDum/FX/FireBall/FireBall/PS_ImpactWallFireBall.PS_ImpactWallFireBall" Hit_Location (`KismetMathLibrary.MakeRotFromYX` Hit_Normal Hit_Normal))
    (set `self.hasHitARat` false)
    (`self.K2_DestroyActor`)))

(event `self.ReceiveDestroyed`
  (bind _returnvalue (`SceneComponent.K2_GetComponentLocation` (`self.Collision`)))
  (if (`self.hasHitARat`)
    (`NiagaraFunctionLibrary.SpawnSystemAtLocation` "/Game/TMPS/TMPS_Art/BaDum/FX/FireBall/FireBall/PS_ImpactRatFireBall_2.PS_ImpactRatFireBall_2" _returnvalue)
    (`NiagaraFunctionLibrary.SpawnSystemAtLocation` "/Game/TMPS/TMPS_Art/BaDum/FX/Death/PS_Death.PS_Death" (+ _returnvalue (0.0 0.0 50.0)))))

(fn `UserConstructionScript`)