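; BP_SwordSwipe is the hit actor for the hero's sword attack, delivering damage through GAS.
; When its collision box overlaps anything but the instigator, the authority applies the stored damage effect spec to character targets' ability systems.
; Rats (BP_baseRat) are destroyed outright instead of damaged.
; The swipe destroys itself on overlap, including on remotes, except when a character target lacks a valid ability system.
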(event `self.BoxCollision.OnComponentBeginOverlap`
  (params (OverlappedComponent :type "PrimitiveComponent Object Reference") (OtherActor :type "Actor Object Reference") (OtherComp :type "PrimitiveComponent Object Reference") (OtherBodyIndex :type Integer) (bFromSweep :type Boolean) (SweepResult :type "HitResult Structure (by ref)"))
  (if (!= OtherActor (`self.GetInstigator`))
    (`/Engine/EditorBlueprintResources/ActorMacros.Switch Has Authority`
      (:`Authority`
        (bind _asbdtcharacter_base (cast `BDTCharacterBase` OtherActor)
          (:`then`
            (bind _returnvalue (`AbilitySystemBlueprintLibrary.GetAbilitySystemComponent` _asbdtcharacter_base))
            (if (`KismetSystemLibrary.IsValid` _returnvalue)
              (`AbilitySystemComponent.BP_ApplyGameplayEffectSpecToSelf` _returnvalue (`self.DamageEffectSpecHandle`))
              (`self.K2_DestroyActor`)))
          (:`CastFailed`
            (bind _asbp_base_rat (cast `/Game/TMPS/BP/BP_baseRat` OtherActor)
              (:`then`
                (`self.K2_DestroyActor` _asbp_base_rat))
              (:`CastFailed`
                _))
            (`self.K2_DestroyActor` :!label _label))))
      (:`Remote`
        (goto _label)))))

(fn `UserConstructionScript`)