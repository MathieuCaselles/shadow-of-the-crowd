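; Manager actor that pre-spawns a pool of Niagara rat particle systems, apparently to visualize rats tracked by BP_BDTGameState.
; BeginPlay caches the game state, then spawns about 2000 PS_Rat systems below the world at Z -1000 and stores them in an array.
; Tick is empty.
; Disconnected nodes retain unused logic for placing systems at spawn height and hiding surplus ones when the rat position count shrinks.
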(event `self.ReceiveBeginPlay`
  (`KismetSystemLibrary.PrintString` "MANAGER")
  (bind _asbp_bdtgame_state (cast `/Game/TMPS/GAS/BP_BDTGameState` (`GameplayStatics.GetGameState`)))
  (set `self.GameState` _asbp_bdtgame_state)
  (for _ (range 2001)
    (bind _returnvalue (`NiagaraFunctionLibrary.SpawnSystemAtLocation` "/Game/TMPS/TMPS_Art/BaDum/FX/Rat/PS_Rat.PS_Rat" (0.0 0.0 -1000.0)))
    (`KismetArrayLibrary.Array_Add` (`self.Niagarats`) _returnvalue)))

(event `self.ReceiveTick`
  (params (DeltaSeconds :type "Float (single-precision)")))

(fn `UserConstructionScript`)