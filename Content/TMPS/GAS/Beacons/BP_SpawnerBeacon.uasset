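; Spawner beacon actor Blueprint in the GAS Beacons folder, currently inert: its events are empty and all logic is disconnected.
; The unwired fragments set a looping timer for SpawnEmitter, clear that timer, and spawn the PS_Cloche effect at the actor's location.
; Another spawns a BP_TokenBeaconSpawner linked back to this beacon, on the Remote branch of an authority switch rather than the Authority one.
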(event `self.ReceiveBeginPlay`)

(event `SpawnToken`)

(event `SpawnEmitter`)

(event `self.ReceiveDestroyed`)

(fn `UserConstructionScript`)