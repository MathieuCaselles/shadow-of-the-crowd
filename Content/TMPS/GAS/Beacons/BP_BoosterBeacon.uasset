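; BP_BoosterBeacon is a booster beacon actor that emits a repeating boost effect and creates a companion token actor.
; On BeginPlay a looping timer spawns the PS_Boost effect attached to its Sphere, and the timer is cleared when the beacon is destroyed.
; BeginPlay also calls SpawnToken, which spawns a BP_TokenBeaconBooster only on the Remote (non-authority) branch, links it back to the beacon and enables its tick.
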(event `SpawnToken`
  (`/Engine/EditorBlueprintResources/ActorMacros.Switch Has Authority`
    (:`Remote`
      (bind _returnvalue (`|SpawnActorFromClass` "/Game/TMPS/BP/BP_TokenBeaconBooster.BP_TokenBeaconBooster_C" (`KismetMathLibrary.MakeTransform` (0.0 0.0 0.0)) "Undefined" "OverrideRootScale" null null))
      (set `/Game/TMPS/BP/BP_TokenBeaconBooster.BeaconBomb` self _returnvalue)
      (`self.SetActorTickEnabled` _returnvalue true))))

(event `self.ReceiveBeginPlay`
  (bind _returnvalue (`KismetSystemLibrary.K2_SetTimerDelegate` (delegate `SpawnEmitter`) 1.8 true))
  (set `self.JeanMichMich` _returnvalue)
  (`self.SpawnToken`))

(event `SpawnEmitter`
  (`NiagaraFunctionLibrary.SpawnSystemAttached` "/Game/TMPS/TMPS_Art/BaDum/FX/Balises/Bp/Balises/Cloche/PS_Boost.PS_Boost" (`self.Sphere`) "None" (0.0 0.0 0.0) (struct) "KeepRelativeOffset"))

(event `self.ReceiveDestroyed`
  (`KismetSystemLibrary.K2_ClearAndInvalidateTimerHandle` (`self.JeanMichMich`)))

(fn `UserConstructionScript`)