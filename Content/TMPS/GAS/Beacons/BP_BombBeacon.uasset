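; Bomb beacon that damages the hero on contact and then destroys itself.
; On BeginPlay it caches the hero and sets its capsule to ignore every BP_EvilWall when moving.
; A hit on the hero applies a GAS damage effect through the beacon's ability system, and destruction spawns a smoke explosion.
; SpawnToken is empty, and the token-spawning logic is disconnected, so it never runs.
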(event `self.ReceiveBeginPlay`
  (bind _returnvalue (`GameplayStatics.GetActorOfClass` "/Script/BaDumTss.BDTHeroCharacter"))
  (set `self.Hero` _returnvalue)
  (bind _outactors (`GameplayStatics.GetAllActorsOfClass` "/Game/TMPS/BP/BP_EvilWall.BP_EvilWall_C"))
  (for _array_element _outactors
    (`PrimitiveComponent.IgnoreActorWhenMoving` (`self.CapsuleComponent`) _array_element true)))

(event `self.ReceiveHit`
  (params (MyComp :type "PrimitiveComponent Object Reference") (Other :type "Actor Object Reference") (OtherComp :type "PrimitiveComponent Object Reference") (bSelfMoved :type Boolean) (HitLocation :type "Vector Structure") (HitNormal :type "Vector Structure") (NormalImpulse :type "Vector Structure") (Hit :type "HitResult Structure (by ref)"))
  ;[1 1 1] Destroy on contact with Hero
  (bind _asbp_hero_character (cast `/Game/TMPS/GAS/BP_HeroCharacter` Other))
  (`AbilitySystemComponent.BP_ApplyGameplayEffectToTarget` :`self` (`self.AbilitySystemComponent`) :`GameplayEffectClass` "/Game/TMPS/GAS/GE_BombBeaconDamage.GE_BombBeaconDamage_C" :`Target` (`AbilitySystemBlueprintLibrary.GetAbilitySystemComponent` _asbp_hero_character))
  (`self.K2_DestroyActor`))

(event `self.ReceiveDestroyed`
  ;[1 1 1] Particle Spawned on destroy
  (`NiagaraFunctionLibrary.SpawnSystemAtLocation` "/Game/TMPS/TMPS_Art/BaDum/FX/Balises/Bp/Balises/Cloche/PS_SmokeExplosion.PS_SmokeExplosion" (`SceneComponent.K2_GetComponentLocation` (`self.Sphere1`)))
  (`ActorComponent.K2_DestroyComponent` (`self.PS_Explosion`)))

(event `SpawnToken`
  ;[1 1 1] SetToken
)

(fn `UserConstructionScript`)