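; BP_BBEGPawn is the player-controlled BBEG pawn, which summons rats and bomb, booster and spawner beacons through the Gameplay Ability System.
; On BeginPlay it grants its Abilities array by index, which Enhanced Input actions activate; releasing rat summon cancels it by tag.
; Possession toggles the Badum UI, and attribute changes relay Energy (normalized), regen rate and Goldus to UI update calls.
; Debug code spawns a rat particle manager on remote clients and prints cursor overlaps.
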(event `SpawnRatsTests`
  ;[1 0.004673 0] DEBUG REPLICATION RAT POSITION
  (bind _asbp_bdtgame_state (cast `/Game/TMPS/GAS/BP_BDTGameState` (`GameplayStatics.GetGameState`)))
  (set `self.BDTGameState` _asbp_bdtgame_state)
  (`/Engine/EditorBlueprintResources/ActorMacros.Switch Has Authority`
    (:`Remote`
      (`KismetSystemLibrary.PrintString` "Spawn de bp manager")
      (`|SpawnActorFromClass` "/Game/TMPS/GAS/BP_ParticlesRatsManager.BP_ParticlesRatsManager_C" (`self.GetTransform`) "Undefined" "OverrideRootScale" null null))))

(event `self.ReceivePossessed`
  (params (NewController :type "Controller Object Reference"))
  ;[1 1 1] FINI
  ;;[1 0.4462 0] ADD UI TO VIEWPORET
  (bind _asplayer_controller (cast `PlayerController` NewController))
  (set `PlayerController.bShowMouseCursor` false _asplayer_controller)
  (`self.CreateBadumUI`))

(event `self.ReceiveBeginPlay`
  ;[1 1 1] FINI
  ;;[0.2578 0 1] Add abilities in bbeg
  (`self.initializeAbilities`)
  ;;[1 0.004673 0] DEBUG TO DELETE
  (`self.SpawnRatsTests`))

(event `CreateBadumUI`
  ;[1 1 1] FINI
  ;;[1 0.4462 0] ADD UI TO VIEWPORET
  (`WidgetLayoutLibrary.RemoveAllWidgets`)
  (bind _returnvalue (`|CreateWidget` "/Game/TMPS/TMPS_Art/BaDum/UI_UX/Badum_UI_controller.Badum_UI_controller_C"))
  (`UserWidget.AddToViewport` _returnvalue 0))

(event `EnhancedInput|/Game/Inputs/BBEGPawn/Actions/IA_SummonRat`
  (params (ActionValue :type Boolean) (ElapsedSeconds :type "Float (double-precision)") (TriggeredSeconds :type "Float (double-precision)") (InputAction :type "InputAction Object Reference" :default "/Game/Inputs/BBEGPawn/Actions/IA_SummonRat.IA_SummonRat"))
  ;[1 1 1] FINI
  ;;[0.2578 0 1] Summon Rats
  (:`Started`
    (`self.ActivateAbility` 0))
  (:`Completed`
    (`self.CancelAbilityWithTags` (struct :`GameplayTags` (struct :`(TagName` "Ability.Skill.Summon.Rats"))))))

(event `self.ReceiveUnpossessed`
  (params (OldController :type "Controller Object Reference"))
  ;[1 1 1] FINI
  ;;[1 0.4462 0] REMOVE UI FROM VIEWPORT
  (`self.RemoveBadumUi`))

(event `RemoveBadumUi`
  ;[1 1 1] FINI
  ;;[1 0.4462 0] REMOVE UI FROM VIEWPORT
  (`WidgetLayoutLibrary.RemoveAllWidgets`))

(event `EnhancedInput|/Game/Inputs/BBEGPawn/Actions/IA_SummonBombBeacon`
  (params (ActionValue :type Boolean) (ElapsedSeconds :type "Float (double-precision)") (TriggeredSeconds :type "Float (double-precision)") (InputAction :type "InputAction Object Reference" :default "/Game/Inputs/BBEGPawn/Actions/IA_SummonBombBeacon.IA_SummonBombBeacon"))
  ;[1 1 1] FINI
  ;;[0.2578 0 1] Summon Bomb Beacon
  (:`Started`
    (`self.ActivateAbility` 1)))

(event `self.OnEnergyChanged`
  (params (oldValue :type "Float (single-precision)") (newValue :type "Float (single-precision)"))
  ;[1 1 1] FINI
  ;;[1 0.4462 0] UPDATE UI Energy
  (`self.BBEGPawnEnergyChanged` (`KismetMathLibrary.FClamp` (/ newValue (`self.GetMaxEnergy`)))))

(event `EnhancedInput|/Game/Inputs/BBEGPawn/Actions/IA_SummonBoosterBeacon`
  (params (ActionValue :type Boolean) (ElapsedSeconds :type "Float (double-precision)") (TriggeredSeconds :type "Float (double-precision)") (InputAction :type "InputAction Object Reference" :default "/Game/Inputs/BBEGPawn/Actions/IA_SummonBoosterBeacon.IA_SummonBoosterBeacon"))
  ;[1 1 1] FINI
  ;;[0.2578 0 1] Summon Booster Beacon
  (:`Started`
    (`self.ActivateAbility` 2)))

(event `self.OnGoldusChanged`
  (params (oldValue :type "Float (single-precision)") (newValue :type "Float (single-precision)"))
  ;[1 1 1] FINI
  ;;[1 0.4462 0] UPDATE UI Goldus
  (`self.BBEGPawnGoldusChanged` newValue))

(event `self.OnEnergyRegenRateChanged`
  (params (oldValue :type "Float (single-precision)") (newValue :type "Float (single-precision)"))
  ;[1 1 1] FINI
  ;;[1 0.4462 0] UPDATE UI Energy Regen Rate
  (`self.BBEGPawnEnergyRegenRateChanged` newValue))

(event `EnhancedInput|/Game/Inputs/BBEGPawn/Actions/IA_SummonSpawnerBeacon`
  (params (ActionValue :type Boolean) (ElapsedSeconds :type "Float (double-precision)") (TriggeredSeconds :type "Float (double-precision)") (InputAction :type "InputAction Object Reference" :default "/Game/Inputs/BBEGPawn/Actions/IA_SummonSpawnerBeacon.IA_SummonSpawnerBeacon"))
  ;[1 1 1] FINI
  ;;[0.2578 0 1] Summon Spawner Beacon
  (:`Started`
    (`self.ActivateAbility` 3)))

(event `self.SMC_Cursor.OnComponentBeginOverlap`
  (params (OverlappedComponent :type "PrimitiveComponent Object Reference") (OtherActor :type "Actor Object Reference") (OtherComp :type "PrimitiveComponent Object Reference") (OtherBodyIndex :type Integer) (bFromSweep :type Boolean) (SweepResult :type "HitResult Structure (by ref)"))
  (`KismetSystemLibrary.PrintString` "OVERLAPPPP"))

(fn `initializeAbilities`
  (for (_array_element _array_index) (`self.Abilities`)
    (`self.GrantAbility` _array_element 1 _array_index)))

(fn `UserConstructionScript`)