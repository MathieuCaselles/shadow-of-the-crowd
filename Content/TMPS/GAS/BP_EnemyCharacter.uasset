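; Player-controlled villain (Badum) character that uses GAS abilities to summon rats, beacons and walls against the hero.
; BeginPlay grants abilities by array index, spawns the hero's safe zone on remote instances and briefly locks input.
; Gated inputs activate abilities by index, while walls spawn as a preview on press and confirm or cancel on release.
; Possession manages the Badum UI, and the server writes its position to GameState as a cursor each tick.
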(event `self.ReceiveTick`
  (params (DeltaSeconds :type "Float (single-precision)"))
  (bind (_returnvalue_x _returnvalue_y) (`KismetMathLibrary.BreakVector` (`self.K2_GetActorLocation`)))
  (`/Engine/EditorBlueprintResources/ActorMacros.Switch Has Authority`
    (:`Authority`
      (`BDTGameState.SetBadumCursorPosition` (`self.GameState`) (`KismetMathLibrary.MakeVector2D` _returnvalue_x _returnvalue_y)))))

(event `SpawnRatsTests`
  ;[1 0.004673 0] DEBUG REPLICATION RAT POSITION
  (bind _asbp_bdtgame_state (cast `/Game/TMPS/GAS/BP_BDTGameState` (`GameplayStatics.GetGameState`)))
  (set `self.BDTGameState` _asbp_bdtgame_state)
  (`/Engine/EditorBlueprintResources/ActorMacros.Switch Has Authority`
    (:`Remote`
      (`|SpawnActorFromClass` "/Game/TMPS/GAS/BP_ParticlesRatsManager.BP_ParticlesRatsManager_C" (`self.GetTransform`) "Undefined" "OverrideRootScale" null null))))

(event `self.ReceiveBeginPlay`
  (bind _returnvalue (`GameplayStatics.GetPlayerController` 0))
  (`self.DisableInput` (`GameplayStatics.GetPlayerController` 0))
  ;[1 1 1] FINI
  (bind _asbp_bdtgame_state (cast `/Game/TMPS/GAS/BP_BDTGameState` (`GameplayStatics.GetGameState`)))
  (set `self.GameState` _asbp_bdtgame_state)
  (bind _returnvalue_2 (`GameplayStatics.GetActorOfClass` "/Game/TMPS/GAS/BP_HeroCharacter.BP_HeroCharacter_C"))
  (set `self.HeroCharacter` _returnvalue_2)
  ;;[0.2578 0 1] Add abilities in bbeg
  (`self.initializeAbilities`)
  (`self.Spawn Safe Zone`)
  (`KismetSystemLibrary.Delay` 1.0)
  (`self.Spawn Safe Zone`)
  (`KismetSystemLibrary.Delay` 5.0)
  (`self.EnableInput` _returnvalue)
  (`self.EnableInput` (`self.HeroCharacter`) _returnvalue))

(event `self.ReceivePossessed`
  (params (NewController :type "Controller Object Reference"))
  ;[1 1 1] FINI
  ;;[1 0.4462 0] ADD UI TO VIEWPORET
  (bind _asplayer_controller (cast `PlayerController` NewController))
  (set `PlayerController.bShowMouseCursor` false _asplayer_controller)
  (`self.CreateBadumUI`))

(event `CreateBadumUI`
  ;[1 1 1] FINI
  ;;[1 0.4462 0] ADD UI TO VIEWPORET
  (`WidgetLayoutLibrary.RemoveAllWidgets`)
  (bind _returnvalue (`|CreateWidget` "/Game/TMPS/TMPS_Art/BaDum/UI_UX/Badum_UI_controller.Badum_UI_controller_C"))
  (bind _output_get (set `self.UIBadum` _returnvalue))
  (`UserWidget.AddToViewport` _returnvalue 0)
  (`UserWidget.AddToViewport` _output_get 0))

(event `EnhancedInput|/Game/Inputs/HeroCharacter/Actions/IA_LightningDash`
  (params (ActionValue :type Boolean) (ElapsedSeconds :type "Float (double-precision)") (TriggeredSeconds :type "Float (double-precision)") (InputAction :type "InputAction Object Reference" :default "/Game/Inputs/HeroCharacter/Actions/IA_LightningDash.IA_LightningDash"))
  ;[1 1 1] FINI
  ;;[0.2578 0 1] Summon Rats
  (:`Triggered`
    (if (`self.bCanUseABblities`)
      (`self.ActivateAbility` 4))))

(event `self.ReceiveUnpossessed`
  (params (OldController :type "Controller Object Reference"))
  ;[1 1 1] FINI
  ;;[1 0.4462 0] REMOVE UI FROM VIEWPORT
  (`self.RemoveBadumUi`))

(event `Spawn Safe Zone`
  ;[0.2578 0 1] Spawn Safe Zone Hero
  (`/Engine/EditorBlueprintResources/ActorMacros.Switch Has Authority`
    (:`Remote`
      ;[1 1 1] FINI
      (`/Engine/EditorBlueprintResources/StandardMacros.IsValid` (`self.ZoneSafeHero`)
        (:`Is Not Valid`
          (bind _returnvalue (`|SpawnActorFromClass` "/Game/TMPS/BP/BP_ZoneSafeHero.BP_ZoneSafeHero_C" (`KismetMathLibrary.MakeTransform` (`self.K2_GetActorLocation` (`self.HeroCharacter`)) (struct) (15.0 15.0 15.0)) "Undefined" "OverrideRootScale" null null))
          (set `self.ZoneSafeHero` _returnvalue))))))

(event `RemoveBadumUi`
  ;[1 1 1] FINI
  ;;[1 0.4462 0] REMOVE UI FROM VIEWPORT
  (`WidgetLayoutLibrary.RemoveAllWidgets`))

(event `EnhancedInput|/Game/Inputs/BBEGPawn/Actions/IA_SummonBombBeacon`
  (params (ActionValue :type Boolean) (ElapsedSeconds :type "Float (double-precision)") (TriggeredSeconds :type "Float (double-precision)") (InputAction :type "InputAction Object Reference" :default "/Game/Inputs/BBEGPawn/Actions/IA_SummonBombBeacon.IA_SummonBombBeacon"))
  ;[1 1 1] FINI
  ;;[0.2578 0 1] Summon Bomb Beacon
  (:`Started`
    (if (`self.bCanUseABblities`)
      (`self.ActivateAbility` 1))))

(event `CustomEvent`
  (params (oldValue :type "Float (single-precision)") (newValue :type "Float (single-precision)"))
  ;[1 1 1] FINI
  ;;[1 0.4462 0] UPDATE UI Energy
)

(event `SpawnPreviewWall`
  ;[0.2578 0 1] SPAWN  PREVIEW WALL
  ;[1 1 1] FINI
  (bind _returnvalue (`|SpawnActorFromClass` "/Game/TMPS/BP/BP_EvilWall.BP_EvilWall_C" (`self.GetTransform`) "AlwaysSpawn" "OverrideRootScale" null self))
  (`self.SetLastWallRep` _returnvalue))

(event `EnhancedInput|/Game/Inputs/BBEGPawn/Actions/IA_SummonBoosterBeacon`
  (params (ActionValue :type Boolean) (ElapsedSeconds :type "Float (double-precision)") (TriggeredSeconds :type "Float (double-precision)") (InputAction :type "InputAction Object Reference" :default "/Game/Inputs/BBEGPawn/Actions/IA_SummonBoosterBeacon.IA_SummonBoosterBeacon"))
  (bind _bcanuseabblities (`self.bCanUseABblities`))
  ;[1 1 1] FINI
  ;;[0.2578 0 1] Summon WALL
  (:`Started`
    (if (and (<= (`self.CurrentWallCooldown`) 0.0) _bcanuseabblities)
      (`self.SpawnPreviewWall`)
      (set `self.bStartSpawnWall` true)))
  (:`Completed`
    (if (and _bcanuseabblities (`self.bStartSpawnWall`))
      (`self.SpawnWall`)
      (`/Game/TMPS/TMPS_Art/BaDum/UI_UX/Badum_UI_controller.LaunchTimerBooster` (`self.UIBadum`))
      (else
        (`self.DestroyWall`)))
    (set `self.bStartSpawnWall` false)))

(event `CustomEvent_1`
  (params (oldValue :type "Float (single-precision)") (newValue :type "Float (single-precision)"))
  ;[1 1 1] FINI
  ;;[1 0.4462 0] UPDATE UI Goldus
)

(event `SetLastWallRep`
  (params (evilWall :type "/Game/TMPS/BP/BP_EvilWall Object Reference"))
  (bind _output_get (set `self.LastWall` evilWall))
  ;[1 1 1] FINI
  (`PrimitiveComponent.IgnoreActorWhenMoving` (`self.CapsuleComponent`) _output_get true))

(event `CustomEvent_2`
  (params (oldValue :type "Float (single-precision)") (newValue :type "Float (single-precision)"))
  ;[1 1 1] FINI
  ;;[1 0.4462 0] UPDATE UI Energy Regen Rate
)

(event `SpawnWall`
  (bind _lastwall (`self.LastWall`))
  ;[1 1 1] FINI
  ;;[0.2578 0 1] SPAWN WALL
  (`/Engine/EditorBlueprintResources/StandardMacros.IsValid` _lastwall
    (:`Is Valid`
      (if (`/Game/TMPS/BP/BP_EvilWall.bWaitingToSpawn` _lastwall)
        (`/Game/TMPS/BP/BP_EvilWall.Spawn Wall` _lastwall)))))

(event `EnhancedInput|/Game/Inputs/BBEGPawn/Actions/IA_SummonSpawnerBeacon`
  (params (ActionValue :type Boolean) (ElapsedSeconds :type "Float (double-precision)") (TriggeredSeconds :type "Float (double-precision)") (InputAction :type "InputAction Object Reference" :default "/Game/Inputs/BBEGPawn/Actions/IA_SummonSpawnerBeacon.IA_SummonSpawnerBeacon"))
  ;[1 1 1] FINI
  ;;[0.2578 0 1] Summon Spawner Beacon
  (:`Started`
    (if (`self.bCanUseABblities`)
      (`self.ActivateAbility` 3))))

(event `DestroyWall`
  (bind _lastwall (`self.LastWall`))
  (`/Engine/EditorBlueprintResources/StandardMacros.IsValid` _lastwall
    (:`Is Valid`
      (if (`/Game/TMPS/BP/BP_EvilWall.bWaitingToSpawn` _lastwall)
        (`self.K2_DestroyActor` _lastwall)))))

(fn `BlockAbilities`
  (set `self.bCanUseABblities` false)
  (`self.CancelAbilityWithTags` (struct :`GameplayTags` (struct :`(TagName` "Ability.Skill.Summon.Rats")))))

(fn `EnableAbilities`
  (set `self.bCanUseABblities` true)
  (`self.ActivateAbility` 0))

(fn `initializeAbilities`
  (for (_array_element _array_index) (`self.Abilities`)
    (`self.GrantAbility` _array_element 1 _array_index)))

(fn `UserConstructionScript`)