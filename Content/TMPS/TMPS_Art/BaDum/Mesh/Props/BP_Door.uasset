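; Portal door that gates the match ending: it opens for the hero once enough KOTH zones are cleared.
; The RotateDoor macro swings both leaves tick by tick, reversing if the hero leaves before completion, then spawns a portal effect.
; Entering the ending box once open triggers HeroWin; HeroLoose handles defeat.
; Both pick victory or defeat widgets by authority, then destroy the session and return to the main menu.
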(event `self.ReceiveBeginPlay`
  (set `self.StartRotationDoor1` (`SceneComponent.K2_GetComponentRotation` (`self.doorportealone1`)))
  (set `self.StartRotationDoor2` (`SceneComponent.K2_GetComponentRotation` (`self.doorportealone2`)))
  (bind _assot_c_game_instance (cast `/Game/TMPS/TMPS_Art/BaDum/UI_UX/SotC_GameInstance` (`GameplayStatics.GetGameInstance`)))
  (set `self.GameInstance` _assot_c_game_instance))

(event `self.Box_KOTH.OnComponentBeginOverlap`
  (params (OverlappedComponent :type "PrimitiveComponent Object Reference") (OtherActor :type "Actor Object Reference") (OtherComp :type "PrimitiveComponent Object Reference") (OtherBodyIndex :type Integer) (bFromSweep :type Boolean) (SweepResult :type "HitResult Structure (by ref)"))
  (bind _gameinstance (`self.GameInstance`))
  (bind _returnvalue_location (`KismetMathLibrary.BreakTransform` (`SceneComponent.K2_GetComponentToWorld` (`self.Door`))))
  (if (and (== OtherActor (`self.HeroCharacter`)) (`self.bHasNotEnded`) (`KismetSystemLibrary.IsValid` _gameinstance) (>= (`/Game/TMPS/TMPS_Art/BaDum/UI_UX/SotC_GameInstance.NumberOfClearedKOTH` _gameinstance) (`self.MaxKOTH`)))
    (`self.RotateDoor` :!label _label
      (:`Ended`
        (bind _returnvalue (`NiagaraFunctionLibrary.SpawnSystemAtLocation` "/Game/TMPS/TMPS_Art/BaDum/FX/Door/PS_PortalDoor.PS_PortalDoor" _returnvalue_location))
        (`KismetSystemLibrary.Delay` 1.0)
        (`NiagaraComponent.SetVariableFloat` _returnvalue "Opacity" 0.0)))))

(event `self.Box_KOTH.OnComponentEndOverlap`
  (params (OverlappedComponent :type "PrimitiveComponent Object Reference") (OtherActor :type "Actor Object Reference") (OtherComp :type "PrimitiveComponent Object Reference") (OtherBodyIndex :type Integer))
  (bind _gameinstance (`self.GameInstance`))
  (if (and (`self.bHasNotEnded`) (== (`self.HeroCharacter`) OtherActor) (`KismetSystemLibrary.IsValid` _gameinstance) (>= (`/Game/TMPS/TMPS_Art/BaDum/UI_UX/SotC_GameInstance.NumberOfClearedKOTH` _gameinstance) (`self.MaxKOTH`)))
    (goto _label :!via `TriggerOut`)))

(event `HeroWin`
  (bind _herocharacter (`self.HeroCharacter`))
  (set `/Game/TMPS/GAS/BP_HeroCharacter.bHasWon` true _herocharacter)
  (`self.K2_DestroyActor` _herocharacter)
  (`self.RedirectToLobby`)
  (`/Engine/EditorBlueprintResources/ActorMacros.Switch Has Authority`
    (:`Authority`
      (bind _returnvalue (`|CreateWidget` "/Game/TMPS/TMPS_Art/BaDum/UI_UX/W_victory.W_victory_C"))
      (`/Engine/EditorBlueprintResources/StandardMacros.IsValid` _returnvalue
        (:`Is Valid`
          _)))
    (:`Remote`
      (bind _returnvalue_2 (`|CreateWidget` "/Game/TMPS/TMPS_Art/BaDum/UI_UX/W_defeat.W_defeat_C"))
      (`/Engine/EditorBlueprintResources/StandardMacros.IsValid` _returnvalue_2
        (:`Is Valid`
          _))))
  (`UserWidget.AddToViewport` _returnvalue_2 0)
  (`UserWidget.AddToViewport` _returnvalue 0))

(event `self.Box_Ending.OnComponentBeginOverlap`
  (params (OverlappedComponent :type "PrimitiveComponent Object Reference") (OtherActor :type "Actor Object Reference") (OtherComp :type "PrimitiveComponent Object Reference") (OtherBodyIndex :type Integer) (bFromSweep :type Boolean) (SweepResult :type "HitResult Structure (by ref)"))
  (if (== OtherActor (`self.HeroCharacter`))
    (if (not (`self.bHasNotEnded`))
      (`/Engine/EditorBlueprintResources/StandardMacros.DoOnce` false
        (:`Completed`
          (`self.HeroWin`))))))

(event `RedirectToLobby`
  (`KismetSystemLibrary.Delay` 5.0)
  (`DestroySessionCallbackProxy.DestroySession` (`GameplayStatics.GetPlayerController` 0)
    (:`OnSuccess`
      (`GameplayStatics.OpenLevel` "Main_menu_level"))))

(event `HeroLoose`
  (`/Engine/EditorBlueprintResources/ActorMacros.Switch Has Authority`
    (:`Authority`
      (bind _returnvalue (`|CreateWidget` "/Game/TMPS/TMPS_Art/BaDum/UI_UX/W_defeat.W_defeat_C"))
      (`/Engine/EditorBlueprintResources/StandardMacros.IsValid` _returnvalue
        (:`Is Valid`
          _)))
    (:`Remote`
      (bind _returnvalue_2 (`|CreateWidget` "/Game/TMPS/TMPS_Art/BaDum/UI_UX/W_victory.W_victory_C"))
      (`/Engine/EditorBlueprintResources/StandardMacros.IsValid` _returnvalue_2
        (:`Is Valid`
          _))))
  (`UserWidget.AddToViewport` _returnvalue 0)
  (`UserWidget.AddToViewport` _returnvalue_2 0)
  (`self.RedirectToLobby`))

(fn `DoRotateDoor`
  (params (Door :type "StaticMeshComponent Object Reference") (FirstRotation :type "Rotator Structure") (RotationValue :type "Rotator Structure") (Left :type Boolean))
  (`SceneComponent.K2_SetWorldRotation` Door (`KismetMathLibrary.RLerp` FirstRotation (`KismetMathLibrary.ComposeRotators` FirstRotation (* RotationValue (`KismetMathLibrary.SelectFloat` 1.0 -1.0 Left))) (`self.Progression`) true) false false))

(fn `UserConstructionScript`)