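; BP_BurnedDecal is a short-lived scorch-mark decal, from the lightning strike FX, that also hurts rats on contact.
; A timeline animates the erosion and emissive parameters of a dynamic decal material created in the construction script, then destroys the actor.
; A capsule overlap damages any BP_baseRat only while CanDamage is set, which a short delay after spawn turns off.
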(event `self.ReceiveBeginPlay`
  (bind _decallightning (`self.DecalLightning`))
  (`|ExecutionSequence`
    (:`then_0`
      (bind (_direction _decal_erosion01 _decal_emissivepower01) (`Timeline|Timeline`)
        (:`Update`
          (`MaterialInstanceDynamic.SetScalarParameterValue` _decallightning "Erosion" _decal_erosion01)
          (`MaterialInstanceDynamic.SetScalarParameterValue` _decallightning "Emissive Scalar" _decal_emissivepower01))
        (:`Finished`
          (`self.K2_DestroyActor`))))
    (:`then_1`
      (`KismetSystemLibrary.Delay` 0.5)
      (set `self.canDamage` false))))

(event `self.Capsule.OnComponentBeginOverlap`
  (params (OverlappedComponent :type "PrimitiveComponent Object Reference") (OtherActor :type "Actor Object Reference") (OtherComp :type "PrimitiveComponent Object Reference") (OtherBodyIndex :type Integer) (bFromSweep :type Boolean) (SweepResult :type "HitResult Structure (by ref)"))
  (if (`self.canDamage`)
    (bind _asbp_base_rat (cast `/Game/TMPS/BP/BP_baseRat` OtherActor))
    (`/Game/TMPS/BP/BP_baseRat.Damage` _asbp_base_rat 1.0)))

(fn `UserConstructionScript`
  (bind _returnvalue (`DecalComponent.CreateDynamicMaterialInstance` (`self.Decal`)))
  (set `self.DecalLightning` _returnvalue))