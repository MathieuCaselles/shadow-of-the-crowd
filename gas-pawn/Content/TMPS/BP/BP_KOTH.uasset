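; BP_KOTH is a King of the Hill capture zone that builds charge while a hero character stands inside it.
; ZoneVisu overlap events toggle IsCharging for BP_HeroCharacter actors, without counting occupants.
; Tick raises Charge at ChargeSpeed or drains it at a slower rate while non-negative, with no upper cap.
; It pushes Charge to its UI_KOTH widget and debug-prints it; Palier threshold checks are unconnected.
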(event `self.ReceiveBeginPlay`
  (bind _asui_koth (cast `/Game/TMPS/BP/TMPS_UI/UI_KOTH` (`WidgetComponent.GetWidget` (`self.Widget`))))
  (set `self.As UI KOTH` _asui_koth))

(event `self.ReceiveTick`
  (params (DeltaSeconds :type "Float (single-precision)"))
  (set `self.Delta Seconds` DeltaSeconds)
  (if (`self.isCharging`)
    (bind _output_get (set `self.Charge` (+ (* (`self.Delta Seconds`) (`self.chargeSpeed`)) (`self.Charge`))))
    (`KismetSystemLibrary.PrintString` (`KismetStringLibrary.Conv_DoubleToString` _output_get) true false (struct :`G` 1.0 :`B` 0.330346 :`A` 1.0) 0.0)
    (set `/Game/TMPS/BP/TMPS_UI/UI_KOTH.charge` _output_get (`self.As UI KOTH`))
    (elif (>= (`self.Charge`) 0.0)
      (bind _output_get_2 (set `self.Charge` (- (`self.Charge`) (* (`self.Delta Seconds`) (`self.chargeSpeed`) 0.7))))
      (`KismetSystemLibrary.PrintString` (`KismetStringLibrary.Conv_DoubleToString` _output_get_2) true false (struct :`R` 1.0 :`B` 0.162127 :`A` 1.0) 0.0)
      (set `/Game/TMPS/BP/TMPS_UI/UI_KOTH.charge` _output_get_2 (`self.As UI KOTH`)))))

(event `self.zoneVisu.OnComponentBeginOverlap`
  (params (OverlappedComponent :type "PrimitiveComponent Object Reference") (OtherActor :type "Actor Object Reference") (OtherComp :type "PrimitiveComponent Object Reference") (OtherBodyIndex :type Integer) (bFromSweep :type Boolean) (SweepResult :type "HitResult Structure (by ref)"))
  (cast `/Game/TMPS/GAS/BP_HeroCharacter` OtherActor)
  (set `self.isCharging` true))

(event `self.zoneVisu.OnComponentEndOverlap`
  (params (OverlappedComponent :type "PrimitiveComponent Object Reference") (OtherActor :type "Actor Object Reference") (OtherComp :type "PrimitiveComponent Object Reference") (OtherBodyIndex :type Integer))
  (cast `/Game/TMPS/GAS/BP_HeroCharacter` OtherActor)
  (set `self.isCharging` false))

(fn `UserConstructionScript`)