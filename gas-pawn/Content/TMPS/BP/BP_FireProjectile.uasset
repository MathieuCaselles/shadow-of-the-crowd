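; Fire projectile that damages rats and bursts against blocking surfaces, destroying itself two seconds after spawning if still alive.
; Sphere overlap with a BP_baseRat calls its Damage function and destroys the projectile.
; Overlap with an actor tagged BLOCK stops movement and spawns a fireball wall-impact effect near the sphere.
; A timeline drives the Niagara erosion and alpha parameters during the brief delay before destruction.
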(event `self.ReceiveBeginPlay`
  (`KismetSystemLibrary.Delay` 2.0)
  (`self.K2_DestroyActor`))

(event `self.Sphere.OnComponentBeginOverlap`
  (params (OverlappedComponent :type "PrimitiveComponent Object Reference") (OtherActor :type "Actor Object Reference") (OtherComp :type "PrimitiveComponent Object Reference") (OtherBodyIndex :type Integer) (bFromSweep :type Boolean) (SweepResult :type "HitResult Structure (by ref)"))
  (bind _niagara (`self.Niagara`))
  (`|ExecutionSequence`
    (:`then_0`
      (bind _asbp_base_rat (cast `/Game/TMPS/BP/BP_baseRat` OtherActor))
      (`/Game/TMPS/BP/BP_baseRat.Damage` _asbp_base_rat 1.0)
      (`self.K2_DestroyActor`))
    (:`then_1`
      (`/Engine/EditorBlueprintResources/StandardMacros.IsValid` self
        (:`Is Valid`
          (if (`self.ActorHasTag` OtherActor "BLOCK")
            (`MovementComponent.StopMovementImmediately` (`self.ProjectileMovement`))
            (`|ExecutionSequence`
              (:`then_0`
                (bind (_direction _erosion _alpha) (`Timeline|Timeline_0` :!via `PlayFromStart`)
                  (:`Update`
                    (`FXSystemComponent.SetFloatParameter` _niagara "Erosion" _erosion)
                    (`FXSystemComponent.SetFloatParameter` _niagara "Alpha" _alpha))))
              (:`then_1`
                (`KismetSystemLibrary.Delay` 0.2)
                (`self.K2_DestroyActor`))
              (:`then_2`
                (`NiagaraFunctionLibrary.SpawnSystemAtLocation` "/Game/TMPS/TMPS_Art/BaDum/FX/FireBall/FireBall/PS_ImpactWallFireBall.PS_ImpactWallFireBall" (+ (`SceneComponent.K2_GetComponentLocation` (`self.Sphere`)) (0.0 -40.0 0.0)))))))))))

(fn `UserConstructionScript`)