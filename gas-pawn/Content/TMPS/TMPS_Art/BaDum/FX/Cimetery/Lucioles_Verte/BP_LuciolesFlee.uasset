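; Cemetery firefly effect Blueprint that makes the fireflies appear to flee when something overlaps its R component.
; On overlap, it switches the point light off and spawns the PS_Lucioles particle system at the static mesh's transform.
; The Lumiere flag blocks retriggering until a short delay ends, when the light returns to a fixed intensity.
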(event `self.ReceiveBeginPlay`
  (set `self.Lumiere?` true))

(event `self.r.OnComponentBeginOverlap`
  (params (OverlappedComponent :type "PrimitiveComponent Object Reference") (OtherActor :type "Actor Object Reference") (OtherComp :type "PrimitiveComponent Object Reference") (OtherBodyIndex :type Integer) (bFromSweep :type Boolean) (SweepResult :type "HitResult Structure (by ref)"))
  (bind (_returnvalue_location _returnvalue_rotation _returnvalue_scale) (`KismetMathLibrary.BreakTransform` (`SceneComponent.K2_GetComponentToWorld` (`self.StaticMesh`))))
  (if (`self.Lumiere?`)
    (set `self.Lumiere?` false)
    (`LightComponent.SetIntensity` (`self.PointLight`) 0.0)
    (`NiagaraFunctionLibrary.SpawnSystemAtLocation` "/Game/TMPS/TMPS_Art/BaDum/FX/Cimetery/Lucioles_Verte/PS_Lucioles.PS_Lucioles" _returnvalue_location _returnvalue_rotation _returnvalue_scale)
    (`KismetSystemLibrary.Delay` 4.0)
    (set `self.Lumiere?` true)
    (`LightComponent.SetIntensity` (`self.PointLight`) 5665.499023)))

(fn `UserConstructionScript`)