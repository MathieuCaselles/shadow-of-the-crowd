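; BP_CircleColumn is a column prop that lights up with purple fire when something overlaps its Collision component.
; Begin overlap raises eight lights' intensity and turns on fire, spark and firefly particles through spawn-rate float parameters.
; End overlap zeroes those values unless Captured is true, so a captured column stays lit.
; Overlaps are not filtered by actor, and Captured is never set in these graphs.
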(event `self.Collision.OnComponentBeginOverlap`
  (params (OverlappedComponent :type "PrimitiveComponent Object Reference") (OtherActor :type "Actor Object Reference") (OtherComp :type "PrimitiveComponent Object Reference") (OtherBodyIndex :type Integer) (bFromSweep :type Boolean) (SweepResult :type "HitResult Structure (by ref)"))
  (bind _ps_fire_purple3 (`self.PS_Fire_purple3`))
  (`LightComponent.SetIntensity` (`self.Light7`) 7500.0)
  (`LightComponent.SetIntensity` (`self.Light5`) 7500.0)
  (`LightComponent.SetIntensity` (`self.Light4`) 7500.0)
  (`LightComponent.SetIntensity` (`self.Light3`) 7500.0)
  (`LightComponent.SetIntensity` (`self.Light2`) 7500.0)
  (`LightComponent.SetIntensity` (`self.Light1`) 7500.0)
  (`LightComponent.SetIntensity` (`self.Light`) 7500.0)
  (`LightComponent.SetIntensity` (`self.Light6`) 7500.0)
  (`FXSystemComponent.SetFloatParameter` _ps_fire_purple3 "SpawnRateFire" 12.0)
  (`FXSystemComponent.SetFloatParameter` (`self.PS_Fire_purple4`) "SpawnRateFire" 12.0)
  (`FXSystemComponent.SetFloatParameter` (`self.PS_Fire_purple5`) "SpawnRateFire" 12.0)
  (`FXSystemComponent.SetFloatParameter` (`self.PS_Fire_purple7`) "SpawnRateFire" 12.0)
  (`FXSystemComponent.SetFloatParameter` (`self.PS_Fire_purple2`) "SpawnRateFire" 12.0)
  (`FXSystemComponent.SetFloatParameter` (`self.PS_Fire_purple6`) "SpawnRateFire" 12.0)
  (`FXSystemComponent.SetFloatParameter` (`self.PS_Fire_purple1`) "SpawnRateFire" 12.0)
  (`FXSystemComponent.SetFloatParameter` (`self.PS_Fire_purple`) "SpawnRateFire" 12.0)
  (`FXSystemComponent.SetFloatParameter` _ps_fire_purple3 "SpawnRateSparks" 20.0)
  (`FXSystemComponent.SetFloatParameter` (`self.PS_Fire_purple4`) "SpawnRateSparks" 20.0)
  (`FXSystemComponent.SetFloatParameter` (`self.PS_Fire_purple2`) "SpawnRateSparks" 20.0)
  (`FXSystemComponent.SetFloatParameter` (`self.PS_Fire_purple7`) "SpawnRateSparks" 20.0)
  (`FXSystemComponent.SetFloatParameter` (`self.PS_Fire_purple6`) "SpawnRateSparks" 20.0)
  (`FXSystemComponent.SetFloatParameter` (`self.PS_Fire_purple5`) "SpawnRateSparks" 20.0)
  (`FXSystemComponent.SetFloatParameter` (`self.PS_Fire_purple`) "SpawnRateSparks" 20.0)
  (`FXSystemComponent.SetFloatParameter` (`self.PS_Fire_purple1`) "SpawnRateSparks" 20.0)
  (`FXSystemComponent.SetFloatParameter` (`self.PS_FireFlys`) "SpawnRate" 8.0))

(event `self.Collision.OnComponentEndOverlap`
  (params (OverlappedComponent :type "PrimitiveComponent Object Reference") (OtherActor :type "Actor Object Reference") (OtherComp :type "PrimitiveComponent Object Reference") (OtherBodyIndex :type Integer))
  (bind _ps_fire_purple3 (`self.PS_Fire_purple3`))
  (if (not (`self.Captured?`))
    (`LightComponent.SetIntensity` (`self.Light7`) 0.0)
    (`LightComponent.SetIntensity` (`self.Light5`) 0.0)
    (`LightComponent.SetIntensity` (`self.Light4`) 0.0)
    (`LightComponent.SetIntensity` (`self.Light3`) 0.0)
    (`LightComponent.SetIntensity` (`self.Light2`) 0.0)
    (`LightComponent.SetIntensity` (`self.Light1`) 0.0)
    (`LightComponent.SetIntensity` (`self.Light`) 0.0)
    (`LightComponent.SetIntensity` (`self.Light6`) 0.0)
    (`FXSystemComponent.SetFloatParameter` _ps_fire_purple3 "SpawnRateFire" 0.0)
    (`FXSystemComponent.SetFloatParameter` (`self.PS_Fire_purple4`) "SpawnRateFire" 0.0)
    (`FXSystemComponent.SetFloatParameter` (`self.PS_Fire_purple5`) "SpawnRateFire" 0.0)
    (`FXSystemComponent.SetFloatParameter` (`self.PS_Fire_purple7`) "SpawnRateFire" 0.0)
    (`FXSystemComponent.SetFloatParameter` (`self.PS_Fire_purple2`) "SpawnRateFire" 0.0)
    (`FXSystemComponent.SetFloatParameter` (`self.PS_Fire_purple6`) "SpawnRateFire" 0.0)
    (`FXSystemComponent.SetFloatParameter` (`self.PS_Fire_purple1`) "SpawnRateFire" 0.0)
    (`FXSystemComponent.SetFloatParameter` (`self.PS_Fire_purple`) "SpawnRateFire" 0.0)
    (`FXSystemComponent.SetFloatParameter` _ps_fire_purple3 "SpawnRateSparks" 0.0)
    (`FXSystemComponent.SetFloatParameter` (`self.PS_Fire_purple4`) "SpawnRateSparks" 0.0)
    (`FXSystemComponent.SetFloatParameter` (`self.PS_Fire_purple2`) "SpawnRateSparks" 0.0)
    (`FXSystemComponent.SetFloatParameter` (`self.PS_Fire_purple7`) "SpawnRateSparks" 0.0)
    (`FXSystemComponent.SetFloatParameter` (`self.PS_Fire_purple6`) "SpawnRateSparks" 0.0)
    (`FXSystemComponent.SetFloatParameter` (`self.PS_Fire_purple5`) "SpawnRateSparks" 0.0)
    (`FXSystemComponent.SetFloatParameter` (`self.PS_Fire_purple`) "SpawnRateSparks" 0.0)
    (`FXSystemComponent.SetFloatParameter` (`self.PS_Fire_purple1`) "SpawnRateSparks" 0.0)
    (`FXSystemComponent.SetFloatParameter` (`self.PS_FireFlys`) "SpawnRate" 0.0)))

(fn `UserConstructionScript`)