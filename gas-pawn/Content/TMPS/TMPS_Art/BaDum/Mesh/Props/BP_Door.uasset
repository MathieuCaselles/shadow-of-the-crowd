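; Two-leaf door prop that slowly slides and rotates apart while the player character is inside its trigger Box.
; Overlap begin drives a Move Component To on each leaf toward fixed relative transforms, and overlap end calls Return on both.
; The position checks on completion do nothing, the emissive Timeline for MC_Door is never triggered, and the 2PointCaptured condition is unconnected.
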(event `self.ReceiveBeginPlay`
  (set `self.Door01Pos` (`SceneComponent.K2_GetComponentLocation` (`self.doorportealone1`)))
  (set `self.Door02Pos` (`SceneComponent.K2_GetComponentLocation` (`self.doorportealone2`))))

(event `self.Box.OnComponentBeginOverlap`
  (params (OverlappedComponent :type "PrimitiveComponent Object Reference") (OtherActor :type "Actor Object Reference") (OtherComp :type "PrimitiveComponent Object Reference") (OtherBodyIndex :type Integer) (bFromSweep :type Boolean) (SweepResult :type "HitResult Structure (by ref)"))
  (if (== OtherActor (`GameplayStatics.GetPlayerCharacter` 0))
    (`|ExecutionSequence`
      (:`then_0`
        (`KismetSystemLibrary.MoveComponentTo` (`self.doorportealone1`) (0.0 -170.395789 19.060411) (struct :`Yaw` 190.0) false false 15.0 :!label _label)
        (if (!= (`self.Door01Pos`) (`SceneComponent.K2_GetComponentLocation` (`self.doorportealone1`)) :`ErrorTolerance` 1.0)
          _))
      (:`then_1`
        (`KismetSystemLibrary.MoveComponentTo` (`self.doorportealone2`) (0.0 174.051479 17.652088) (struct :`Yaw` -10.0) false false 15.0 :!label _label_2)
        (if (!= (`self.Door02Pos`) (`SceneComponent.K2_GetComponentLocation` (`self.doorportealone2`)) :`ErrorTolerance` 1.0)
          _)))))

(event `self.Box.OnComponentEndOverlap`
  (params (OverlappedComponent :type "PrimitiveComponent Object Reference") (OtherActor :type "Actor Object Reference") (OtherComp :type "PrimitiveComponent Object Reference") (OtherBodyIndex :type Integer))
  (if (== (`GameplayStatics.GetPlayerCharacter` 0) OtherActor)
    (`|ExecutionSequence`
      (:`then_0`
        (goto _label :!via `Return`))
      (:`then_1`
        (goto _label_2 :!via `Return`)))))

(fn `UserConstructionScript`)