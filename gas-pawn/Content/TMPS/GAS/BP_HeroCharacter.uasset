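; Playable hero character that uses the Gameplay Ability System for fireball summoning, a sword attack and a lightning dash.
; On BeginPlay it grants each entry in its Abilities array with the index as input code, and Enhanced Input actions activate them by index, with fireball release cancelling by tag.
; A debug key spawns and possesses a BBEG pawn.
; Older dash, tilt-shift depth-of-field and direction-widget logic remains disconnected.
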(event `Key|SpaceBar`
  (params (Key :type "Key Structure"))
  ;[1 0.873 0.01239] TMPS DEBUG SWITCH TO BADUM
  (:`Pressed`
    (bind _returnvalue (`|SpawnActorFromClass` "/Game/TMPS/GAS/BP_BBEGPawn.BP_BBEGPawn_C" (`KismetMathLibrary.MakeTransform` (`SceneComponent.K2_GetComponentLocation` (`self.CapsuleComponent`))) "Undefined" "OverrideRootScale" null null :!label _label))
    (`Controller.Possess` (`GameplayStatics.GetPlayerController` 0) _returnvalue)))

(event `Key|Gamepad_Special_Left`
  (params (Key :type "Key Structure"))
  ;[1 0.873 0.01239] TMPS DEBUG SWITCH TO BADUM
  (:`Pressed`
    (goto _label)))

(event `self.ReceivePossessed`
  (params (NewController :type "Controller Object Reference"))
  ;[1 1 1] TMPS IMPORT HERO BLUEPRINT
)

(event `self.ReceiveBeginPlay`
  ;[1 1 1] Ne bouge plus
  ;;[0.2578 0 1] Add abilities in hero
  (`self.initializeAbilities`))

(event `EnhancedInput|/Game/Inputs/HeroCharacter/Actions/IA_SummonFireBall`
  (params (ActionValue :type Boolean) (ElapsedSeconds :type "Float (double-precision)") (TriggeredSeconds :type "Float (double-precision)") (InputAction :type "InputAction Object Reference" :default "/Game/Inputs/HeroCharacter/Actions/IA_SummonFireBall.IA_SummonFireBall"))
  ;[1 1 1] Ne bouge plus
  ;;[0.2578 0 1] Summon Fireball
  (:`Triggered`
    (`self.ActivateAbility` 0))
  (:`Completed`
    (`self.CancelAbilityWithTags` (struct :`GameplayTags` (struct :`(TagName` "Ability.Skill.SummonFireBall"))))))

(event `EnhancedInput|/Game/Inputs/HeroCharacter/Actions/IA_AttackWithSword`
  (params (ActionValue :type Boolean) (ElapsedSeconds :type "Float (double-precision)") (TriggeredSeconds :type "Float (double-precision)") (InputAction :type "InputAction Object Reference" :default "/Game/Inputs/HeroCharacter/Actions/IA_AttackWithSword.IA_AttackWithSword"))
  ;[1 1 1] Ne bouge plus
  ;;[0.2578 0 1] Attack With Sword
  (:`Started`
    (`self.ActivateAbility` 1)))

(event `EnhancedInput|/Game/Inputs/HeroCharacter/Actions/IA_LightningDash`
  (params (ActionValue :type Boolean) (ElapsedSeconds :type "Float (double-precision)") (TriggeredSeconds :type "Float (double-precision)") (InputAction :type "InputAction Object Reference" :default "/Game/Inputs/HeroCharacter/Actions/IA_LightningDash.IA_LightningDash"))
  ;[1 1 1] Ne bouge plus
  ;;[0.2578 0 1] Lightning Dash
  (:`Started`
    (`self.ActivateAbility` 2)))

(event `Key|Gamepad_FaceButton_Left`
  (params (Key :type "Key Structure"))
  ;[1 1 1] TMPS IMPORT HERO BLUEPRINT
  ;;[0.2578 0 1] Dash
)

(event `Key|Gamepad_FaceButton_Right`
  (params (Key :type "Key Structure"))
  ;[1 1 1] TMPS IMPORT HERO BLUEPRINT
  ;;[0.2578 0 1] Dash
)

(event `Key|LeftShift`
  (params (Key :type "Key Structure"))
  ;[1 1 1] TMPS IMPORT HERO BLUEPRINT
  ;;[0.2578 0 1] Dash
)

(fn `initializeAbilities`
  (for (_array_element _array_index) (`self.Abilities`)
    (`self.GrantAbility` _array_element 1 _array_index)))

(fn `UserConstructionScript`)