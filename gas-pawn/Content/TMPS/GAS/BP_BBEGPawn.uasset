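; BP_BBEGPawn is a pawn that shadows the Hero actor and offers a temporary debug switch to controlling it.
; On BeginPlay and every Tick it looks up the Hero by class and moves to its location with a sweep, printing "Oskour" if none exists.
; Space Bar or Gamepad Special Left makes player controller 0 possess the Hero, then destroys this pawn.
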(event `self.ReceiveTick`
  (params (DeltaSeconds :type "Float (single-precision)"))
  (bind _returnvalue (`GameplayStatics.GetActorOfClass` (`self.Hero`) :!label _label))
  (`/Engine/EditorBlueprintResources/StandardMacros.IsValid` _returnvalue
    (:`Is Valid`
      (`self.K2_SetActorLocation` (`self.K2_GetActorLocation` _returnvalue) true))
    (:`Is Not Valid`
      (`KismetSystemLibrary.PrintString` "Oskour"))))

(event `self.ReceiveBeginPlay`
  (goto _label))

(event `Key|SpaceBar`
  (params (Key :type "Key Structure"))
  ;[1 0.873 0.01239] TMPS DEBUG SWITCH TO BADUM
  (:`Pressed`
    (bind _returnvalue (`GameplayStatics.GetActorOfClass` (`self.Hero`) :!label _label_2))
    (`Controller.Possess` (`GameplayStatics.GetPlayerController` 0) _returnvalue)
    (`self.K2_DestroyActor`)))

(event `Key|Gamepad_Special_Left`
  (params (Key :type "Key Structure"))
  ;[1 0.873 0.01239] TMPS DEBUG SWITCH TO BADUM
  (:`Pressed`
    (goto _label_2)))

(fn `UserConstructionScript`)